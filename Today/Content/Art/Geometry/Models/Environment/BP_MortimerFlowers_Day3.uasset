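; Day 3 flower receptacle for Mortimer that collects three flower actors and updates Mortimer's dialogue.
; Box overlaps count each BP_Day3_Flower, snap its mesh to the socket matching the count and disable its collision; end overlaps decrement the count.
; The third flower sets NPC_Mortimer_Day3's Response to Conversation_Mortimer.
; Separately, Tick sets Finished and the same Response whenever the Magazine, Sticky and Letters flags are all true.
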(event OnComponentBeginOverlap(Box)
  (params (OverlappedComponent :type Primitive%20Component%20Object%20Reference) (OtherActor :type Actor%20Object%20Reference) (OtherComp :type Primitive%20Component%20Object%20Reference) (OtherBodyIndex :type Integer) (bFromSweep :type Boolean) (SweepResult :type Hit%20Result%20Structure%20%28by%20ref%29))
  (bind _asbp_day_3_flower (Utilities|Casting|CastToBP_Day3_Flower OtherActor))
  (Variables|Default|SetAddingFlower _asbp_day_3_flower)
  (Variables|Default|SetFlowers%20Inside%20Box (+ (Variables|Default|GetFlowers%20Inside%20Box) 1))
  (switch int (Variables|Default|GetFlowers%20Inside%20Box)
    (:1
      ;[1 1 1] Flower 1
      (Transformation|AttachComponentToComponent (Variables|/Game/Blueprints/Inventory/Items/Item.Item_C|GetStatic%20Mesh%20%28Item%29 (Variables|Default|GetAddingFlower)) (Variables|/Script/Engine.StaticMeshActor|GetStaticMeshComponent self) "Flower 1" "SnapToTarget" "KeepRelative" "KeepRelative" true))
    (:2
      ;[1 1 1] Flower 2
      (Transformation|AttachComponentToComponent (Variables|/Game/Blueprints/Inventory/Items/Item.Item_C|GetStatic%20Mesh%20%28Item%29 (Variables|Default|GetAddingFlower)) (Variables|/Script/Engine.StaticMeshActor|GetStaticMeshComponent self) "Flower 2" "SnapToTarget" "KeepRelative" "KeepRelative" true))
    (:3
      ;[1 1 1] Flower 3
      (Transformation|AttachComponentToComponent (Variables|/Game/Blueprints/Inventory/Items/Item.Item_C|GetStatic%20Mesh%20%28Item%29 (Variables|Default|GetAddingFlower)) (Variables|/Script/Engine.StaticMeshActor|GetStaticMeshComponent self) "Flower 3" "SnapToTarget" "KeepRelative" "KeepRelative" true)))
  (Collision|SetActorEnableCollision (Variables|Default|GetAddingFlower) false)
  (Variables|Default|SetAddingFlower 0)
  (if (== (Variables|Default|GetFlowers%20Inside%20Box) 3)
    (bind _returnvalue (Actor|GetActorOfClass "/Game/Blueprints/NPC/NPC_Mortimer_Day3.NPC_Mortimer_Day3_C"))
    (Variables|/Game/Blueprints/NPC/NPC_Base.NPC_Base_C|SetResponse _returnvalue "Conversation_Mortimer")))

(event OnComponentEndOverlap(Box)
  (params (OverlappedComponent :type Primitive%20Component%20Object%20Reference) (OtherActor :type Actor%20Object%20Reference) (OtherComp :type Primitive%20Component%20Object%20Reference) (OtherBodyIndex :type Integer))
  (Utilities|Casting|CastToBP_Day3_Flower OtherActor)
  (Variables|Default|SetFlowers%20Inside%20Box (- (Variables|Default|GetFlowers%20Inside%20Box) 1)))

(event EventBeginPlay
  (Variables|Default|SetFlowers%20Inside%20Box 0))

(event Collision|EventActorBeginOverlap
  (params (OtherActor :type Actor%20Object%20Reference)))

(event EventTick
  (params (DeltaSeconds :type Float%20%28single-precision%29))
  (if (Math|Boolean|ANDBoolean (Variables|Default|GetMagazine) (Variables|Default|GetSticky) (Variables|Default|GetLetters))
    (Variables|Default|SetFinished true)
    (bind _returnvalue (Actor|GetActorOfClass "/Game/Blueprints/NPC/NPC_Mortimer_Day3.NPC_Mortimer_Day3_C"))
    (Variables|/Game/Blueprints/NPC/NPC_Base.NPC_Base_C|SetResponse _returnvalue "Conversation_Mortimer")))

(fn ConstructionScript)