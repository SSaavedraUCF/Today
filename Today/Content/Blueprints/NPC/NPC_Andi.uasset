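; Blueprint for the NPC Andi, whose Talk event opens a dialogue suited to the current Response state.
; It sets the avatar and name on the game mode's HUD dialog box and removes the interact prompt.
; A switch on Response assigns a stage-specific dialogue tree (start, jump, watering, garbage) to its NPC_AI controller, which starts the dialogue.
; A "forgot" tree assignment is left unreachable.
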(event EventBeginPlay
  (|CallParentFunction) ; This node is disabled and will not be called.\nDrag off pins to build functionality.
)

(event Collision|EventActorBeginOverlap
  (params (OtherActor :type Actor%20Object%20Reference)))

(event EventTick
  (params (DeltaSeconds :type Float%20%28single-precision%29))
  (|CallParentFunction DeltaSeconds) ; This node is disabled and will not be called.\nDrag off pins to build functionality.
)

(event EventTalk
  (bind _asthird_person_game_mode (Utilities|Casting|CastToThirdPersonGameMode (Game|GetGameMode)))
  (Appearance|SetBrushfromTexture (Variables|/Game/Blueprints/Dialogue/Widgets/W_DialoguePH.W_DialoguePH_C|GetNPCAvatar (Variables|/Game/Blueprints/Inventory/InventoryUI/UI_HUD.UI_HUD_C|GetDialogBox (Variables|/Game/PlayerBP/Blueprints/ThirdPersonGameMode.ThirdPersonGameMode_C|GetHeads%20Up%20Display _asthird_person_game_mode))) (Variables|Default|GetSet%20Avatar) false)
  (Variables|/Game/Blueprints/Dialogue/Widgets/W_DialoguePH.W_DialoguePH_C|SetNameText (Variables|/Game/Blueprints/Inventory/InventoryUI/UI_HUD.UI_HUD_C|GetDialogBox (Variables|/Game/PlayerBP/Blueprints/ThirdPersonGameMode.ThirdPersonGameMode_C|GetHeads%20Up%20Display _asthird_person_game_mode)) (Variables|Default|GetsetNameText))
  (Widget|RemovefromParent (Variables|Default|GetInteractText))
  (Variables|Default|SetInteractText 0)
  (bind _asnpc_ai (Utilities|Casting|CastToNPC_AI (AI|GetAIController self)))
  (switch name (Variables|Default|GetResponse)
    (:Default
      (Variables|/Game/Blueprints/Dialogue/NPC_AI.NPC_AI_C|SetDialogueTree _asnpc_ai "/Game/Blueprints/Dialogue/Dialogue_Trees/Andi/Tutorial/T_Andi_Start.T_Andi_Start"))
    (:Start
      (Variables|/Game/Blueprints/Dialogue/NPC_AI.NPC_AI_C|SetDialogueTree _asnpc_ai "/Game/Blueprints/Dialogue/Dialogue_Trees/Andi/Tutorial/T_Andi_Start.T_Andi_Start"))
    (:WaitJump
      (Variables|/Game/Blueprints/Dialogue/NPC_AI.NPC_AI_C|SetDialogueTree _asnpc_ai "/Game/Blueprints/Dialogue/Dialogue_Trees/Andi/Tutorial/T_Andi_WaitJump.T_Andi_WaitJump"))
    (:Jumped
      (Variables|/Game/Blueprints/Dialogue/NPC_AI.NPC_AI_C|SetDialogueTree _asnpc_ai "/Game/Blueprints/Dialogue/Dialogue_Trees/Andi/Tutorial/andi2dialogue/T_Andi_Jump.T_Andi_Jump"))
    (:WaterWait
      (Variables|/Game/Blueprints/Dialogue/NPC_AI.NPC_AI_C|SetDialogueTree _asnpc_ai "/Game/Blueprints/Dialogue/Dialogue_Trees/Andi/Tutorial/T_Andi_WaterWait.T_Andi_WaterWait"))
    (:Watered
      (Variables|/Game/Blueprints/Dialogue/NPC_AI.NPC_AI_C|SetDialogueTree _asnpc_ai "/Game/Blueprints/Dialogue/Dialogue_Trees/Andi/Tutorial/andi2dialogue/Dialogue_Tree_FinalDialogue.Dialogue_Tree_FinalDialogue"))
    (:WaterGarbage
      (Variables|/Game/Blueprints/Dialogue/NPC_AI.NPC_AI_C|SetDialogueTree _asnpc_ai "/Game/Blueprints/Dialogue/Dialogue_Trees/Andi/Tutorial/andi2dialogue/Dialogue_Tree_watering_garbage.Dialogue_Tree_watering_garbage")))
  (Default|StartDialogue _asnpc_ai))

(fn ConstructionScript
  (|CallParentFunction))