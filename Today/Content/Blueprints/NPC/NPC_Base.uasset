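; Base NPC Blueprint that starts a dialogue with the player through its NPC_AI controller.
; BeginPlay passes a default dialogue tree to the controller; Talk swaps in a StartCube tree based on the Response state, then starts dialogue.
; Box overlap creates an interact prompt widget, but adding it to the viewport and end-overlap removal are disconnected.
; DialogueCreate and DialogueGetLine implement CSV data-table dialogue, uncalled here, with their row-gathering step disconnected.
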(event OnComponentBeginOverlap(Box)
  (params (OverlappedComponent :type Primitive%20Component%20Object%20Reference) (OtherActor :type Actor%20Object%20Reference) (OtherComp :type Primitive%20Component%20Object%20Reference) (OtherBodyIndex :type Integer) (bFromSweep :type Boolean) (SweepResult :type Hit%20Result%20Structure%20%28by%20ref%29))
  (Utilities|Casting|CastToPlayerBP OtherActor)
  (bind _returnvalue (UserInterface|CreateWidget "/Game/Blueprints/Inventory/Interact_Text.Interact_Text_C" (Game|GetPlayerController 0) "Press E to Interact"))
  (bind _output_get (Variables|Default|SetInteractText _returnvalue)))

(event OnComponentEndOverlap(Box)
  (params (OverlappedComponent :type Primitive%20Component%20Object%20Reference) (OtherActor :type Actor%20Object%20Reference) (OtherComp :type Primitive%20Component%20Object%20Reference) (OtherBodyIndex :type Integer)))

(event EventBeginPlay
  (bind _asnpc_ai (Utilities|Casting|CastToNPC_AI (AI|GetAIController self)))
  (Variables|/Game/Blueprints/Dialogue/NPC_AI.NPC_AI_C|SetDialogueTree _asnpc_ai (Variables|Default|GetDialogueTree)))

(event EventTalk
  (Widget|RemovefromParent (Variables|Default|GetInteractText))
  (Variables|Default|SetInteractText 0)
  (bind _asnpc_ai (Utilities|Casting|CastToNPC_AI (AI|GetAIController self)))
  (switch name (Variables|Default|GetResponse)
    (:Default
      (Variables|/Game/Blueprints/Dialogue/NPC_AI.NPC_AI_C|SetDialogueTree _asnpc_ai "/Game/Blueprints/Dialogue/Dialogue_Trees/Prototype/StartCube_Start.StartCube_Start" :!label _label))
    (:Start
      (goto _label))
    (:FlowerStart
      (Variables|/Game/Blueprints/Dialogue/NPC_AI.NPC_AI_C|SetDialogueTree _asnpc_ai "/Game/Blueprints/Dialogue/Dialogue_Trees/Prototype/StartCube_Flowers.StartCube_Flowers"))
    (:Watered!
      (Variables|/Game/Blueprints/Dialogue/NPC_AI.NPC_AI_C|SetDialogueTree _asnpc_ai "/Game/Blueprints/Dialogue/Dialogue_Trees/Prototype/StartCube_Trash.StartCube_Trash"))
    (:WaitTrash
      (Variables|/Game/Blueprints/Dialogue/NPC_AI.NPC_AI_C|SetDialogueTree _asnpc_ai "/Game/Blueprints/Dialogue/Dialogue_Trees/Prototype/StartCube_WaitTrash.StartCube_WaitTrash"))
    (:Trashed
      (Variables|/Game/Blueprints/Dialogue/NPC_AI.NPC_AI_C|SetDialogueTree _asnpc_ai "/Game/Blueprints/Dialogue/Dialogue_Trees/Prototype/StartCube_Trashed.StartCube_Trashed"))
    (:Finished
      (Variables|/Game/Blueprints/Dialogue/NPC_AI.NPC_AI_C|SetDialogueTree _asnpc_ai "/Game/Blueprints/Dialogue/Dialogue_Trees/Prototype/StartCube_Finished.StartCube_Finished"))
    (:Dream
      (Variables|/Game/Blueprints/Dialogue/NPC_AI.NPC_AI_C|SetDialogueTree _asnpc_ai "/Game/Blueprints/Dialogue/Dialogue_Trees/Prototype/StartCube_Dream.StartCube_Dream")))
  (Default|StartDialogue _asnpc_ai))

(event EventTick
  (params (DeltaSeconds :type Float%20%28single-precision%29)))

(fn ConstructionScript)

(fn DialogueCreate
  ;[1 1 1] Checks to see if Widget is there
  (Utilities|IsValid (Variables|Default|GetDialogueBox)
    (:Is%20Valid
      ;[1 1 1] If widget is there, add text
      (bind _returnedline (CallFunction|DialogueGetLine))
      (if (not (Utilities|Text|TextIsEmpty _returnedline))
        (Variables|/Game/Blueprints/Dialogue/Widgets/W_DialoguePH.W_DialoguePH_C|SetDialogueText (Variables|Default|GetDialogueBox) _returnedline)))
    (:Is%20Not%20Valid
      ;[1 1 1] Adds widget to the player's screen
      (bind _returnvalue (UserInterface|CreateWidget "/Game/Blueprints/Dialogue/Widgets/W_DialoguePH.W_DialoguePH_C" (Game|GetPlayerController 0)))
      (bind _output_get (Variables|Default|SetDialogueBox _returnvalue))
      (UserInterface|Viewport|AddtoViewport _output_get 0)
      (bind _returnedline_2 (CallFunction|DialogueGetLine))
      (Variables|/Game/Blueprints/Dialogue/Widgets/W_DialoguePH.W_DialoguePH_C|SetDialogueText (Variables|Default|GetDialogueBox) _returnedline_2)
      (Variables|/Game/Blueprints/Dialogue/Widgets/W_DialoguePH.W_DialoguePH_C|SetNameText (Variables|Default|GetDialogueBox) (Variables|Default|GetsetNameText)))))

(fn DialogueGetLine
  (for _array_element (Variables|Default|GetMyDialogue)
    (bind _returnvalue (Utilities|GetDataTableRow "/Game/Blueprints/Dialogue/Old_Dialogue/CSV_TestDialogue.CSV_TestDialogue" _array_element)
      (:then
        (if (and (== (.Conversation_ID (Utilities|Struct|BreakDialogueStructure _returnvalue)) (Variables|Default|GetConversation_ID)) (== (.Line_ID (Utilities|Struct|BreakDialogueStructure _returnvalue)) (Variables|Default|GetLineCurrent)))
          (Utilities|Array|Add (LocalVariables|GetReturnedLines) (.Dialogue (Utilities|Struct|BreakDialogueStructure _returnvalue)))))))
  (if (== (Utilities|Array|Length (LocalVariables|GetReturnedLines)) 1)
    (return (Utilities|Array|Get(acopy) (LocalVariables|GetReturnedLines)))
    (else
      (Widget|RemovefromParent (Variables|Default|GetDialogueBox))
      (Variables|Default|SetDialogueBox 0)
      (Variables|Default|SetLineCurrent 0))))