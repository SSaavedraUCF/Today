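; NPC Blueprint for Whitney on day 7 that opens her neighborhood conversation when talked to.
; The Talk event puts her name in the HUD dialog box via the game mode and removes the interact prompt.
; It then hands the Day_7_neighborhood dialogue tree to its NPC_AI controller and starts the dialogue.
; BeginPlay, overlap, Tick and the construction script add no logic of their own.
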(event EventBeginPlay
  (|CallParentFunction) ; This node is disabled and will not be called.\nDrag off pins to build functionality.
)

(event Collision|EventActorBeginOverlap
  (params (OtherActor :type Actor%20Object%20Reference))
  (|CallParentFunction OtherActor) ; This node is disabled and will not be called.\nDrag off pins to build functionality.
)

(event EventTalk
  (bind _asthird_person_game_mode (Utilities|Casting|CastToThirdPersonGameMode (Game|GetGameMode)))
  (Variables|/Game/Blueprints/Dialogue/Widgets/W_DialoguePH.W_DialoguePH_C|SetNameText (Variables|/Game/Blueprints/Inventory/InventoryUI/UI_HUD.UI_HUD_C|GetDialogBox (Variables|/Game/PlayerBP/Blueprints/ThirdPersonGameMode.ThirdPersonGameMode_C|GetHeads%20Up%20Display _asthird_person_game_mode)) (Variables|Default|GetsetNameText))
  (Widget|RemovefromParent (Variables|Default|GetInteractText))
  (Variables|Default|SetInteractText 0)
  (bind _asnpc_ai (Utilities|Casting|CastToNPC_AI (AI|GetAIController self)))
  (switch name (Variables|Default|GetResponse)
    (:Default
      (Variables|/Game/Blueprints/Dialogue/NPC_AI.NPC_AI_C|SetDialogueTree _asnpc_ai "/Game/Blueprints/Dialogue/Dialogue_Trees/Day7/Day_7_neighborhood.Day_7_neighborhood")
      (Default|StartDialogue _asnpc_ai))))

(event EventTick
  (params (DeltaSeconds :type Float%20%28single-precision%29)))

(fn ConstructionScript
  (|CallParentFunction))