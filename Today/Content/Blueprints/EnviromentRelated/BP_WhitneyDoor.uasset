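; BP_WhitneyDoor is a swinging door that shows a "Press O to Use Door" prompt while Player_Eve overlaps it.
; Overlap events add or remove the prompt widget and track the Interactable flag.
; The Opening event drives a timeline that rotates Anchor's yaw, reversing only when both Interactable and Opened are true.
; Its NAND check lets the door open even when not interactable; no input binding appears here.
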(event EventBeginPlay)

(event Collision|EventActorBeginOverlap
  (params (OtherActor :type Actor%20Object%20Reference))
  (Utilities|Casting|CastToPlayer_Eve OtherActor)
  (Variables|Default|SetInteractable? true)
  (bind _returnvalue (UserInterface|CreateWidget "/Game/Blueprints/Inventory/Widgets/Interact_Text.Interact_Text_C" 0 "Press O to Use Door")) ; Change Key
  (bind _output_get (Variables|Default|SetInteract%20Text _returnvalue))
  (UserInterface|Viewport|AddtoViewport _output_get 0))

(event EventTick
  (params (DeltaSeconds :type Float%20%28single-precision%29)))

(event EventOpening
  (params (Actor :type Actor%20Object%20Reference))
  (if (Math|Boolean|NANDBoolean (Variables|Default|GetInteractable?) (Variables|Default|GetOpened?))
    (Variables|Default|SetOpened? true)
    (bind _rotation (Timeline|Open%20TL Play)
      (:Update
        (Transformation|SetRelativeRotation (Variables|Default|GetAnchor) (Math|Rotator|MakeRotator 0.0 0.0 _rotation) false false)))
    (else
      (Variables|Default|SetOpened? false)
      (Timeline|Open%20TL Reverse))))

(event Collision|EventActorEndOverlap
  (params (OtherActor :type Actor%20Object%20Reference))
  (bind _interact_text (Variables|Default|GetInteract%20Text)
    (:then
      (Widget|RemovefromParent _interact_text)
      (Variables|Default|SetInteract%20Text 0)
      (Utilities|Casting|CastToPlayer_Eve OtherActor)
      (Variables|Default|SetInteractable? false))
    (:else)))

(fn ConstructionScript)