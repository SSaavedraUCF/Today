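; BP_DoorTele_Condition is a teleport door variant that only offers entry once Eve has finished talking to Whitney on Day 6.
; On box overlap it finds the NPC_Day6_WhitneyStart actor and checks that its Response is "Interacted".
; If so and the overlapping actor is Player_Eve, it shows a "Left Click to Enter" prompt and sets Interactable.
; The Opening event simply defers to the parent class.
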(event OnComponentBeginOverlap(Box)
  (params (OverlappedComponent :type Primitive%20Component%20Object%20Reference) (OtherActor :type Actor%20Object%20Reference) (OtherComp :type Primitive%20Component%20Object%20Reference) (OtherBodyIndex :type Integer) (bFromSweep :type Boolean) (SweepResult :type Hit%20Result%20Structure%20%28by%20ref%29))
  ;[1 1 1] Checking if eve finished talking to withney
  (bind _returnvalue (Actor|GetActorOfClass "/Game/Blueprints/NPC/Day6/NPC_Day6_WhitneyStart.NPC_Day6_WhitneyStart_C"))
  (if (Utilities|Name|Equal(Name) (Variables|/Game/Blueprints/NPC/NPC_Base.NPC_Base_C|GetResponse _returnvalue) "Interacted")
    (Utilities|Casting|CastToPlayer_Eve OtherActor)
    (bind _returnvalue_2 (UserInterface|CreateWidget "/Game/Blueprints/Inventory/Widgets/Interact_Text.Interact_Text_C" 0 "Left Click to Enter"))
    (bind _output_get (Variables|Default|SetInteract%20Text _returnvalue_2))
    (UserInterface|Viewport|AddtoViewport _output_get 0)
    (Variables|Default|SetInteractable? true)))

(event EventBeginPlay
  (|CallParentFunction) ; This node is disabled and will not be called.\nDrag off pins to build functionality.
)

(event EventTick
  (params (DeltaSeconds :type Float%20%28single-precision%29))
  (|CallParentFunction DeltaSeconds) ; This node is disabled and will not be called.\nDrag off pins to build functionality.
)

(event EventOpening
  (params (Actor :type Actor%20Object%20Reference))
  (|CallParentFunction 0))

(fn ConstructionScript
  (|CallParentFunction))