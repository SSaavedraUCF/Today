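; Boundary warning trigger actor that shows a dialogue line from Eve when the Player_Eve character overlaps it.
; On overlap it creates a W_DialoguePH widget with configurable text and avatar, then disables player input.
; Tick polls the E key to close the box and restore input, destroying the actor if DisplayOnce is set.
; A character ending overlap also removes the box.
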(event EventTick
  (params (DeltaSeconds :type Float%20%28single-precision%29))
  ;[1 1 1] Destroy the box text if the player press e
  (bind _dialoguebox (Variables|Default|GetDialogueBox)
    (:then
      (if (Game|Player|WasInputKeyJustPressed (Game|GetPlayerController 0) "E")
        (Widget|RemovefromParent _dialoguebox)
        (Input|EnableInput (Game|GetPlayerCharacter 0) (Game|GetPlayerController 0))
        (if (Variables|Default|GetDisplayOnce)
          (Actor|DestroyActor))))
    (:else)))

(event Collision|EventActorBeginOverlap
  (params (OtherActor :type Actor%20Object%20Reference))
  ;[1 1 1] Pop up the dialog when player collide with the collider
  (Utilities|Casting|CastToPlayer_Eve OtherActor)
  (bind _returnvalue (UserInterface|CreateWidget "/Game/Blueprints/Dialogue/Widgets/W_DialoguePH.W_DialoguePH_C"))
  (bind _output_get (Variables|Default|SetDialogueBox _returnvalue))
  (Variables|/Game/Blueprints/Dialogue/Widgets/W_DialoguePH.W_DialoguePH_C|SetNameText _output_get "Eve")
  (Variables|/Game/Blueprints/Dialogue/Widgets/W_DialoguePH.W_DialoguePH_C|SetDialogueText _output_get (Variables|Default|GetBox%20Text))
  (Variables|/Game/Blueprints/Dialogue/Widgets/W_DialoguePH.W_DialoguePH_C|SetAvatarImage _output_get (Variables|Default|GetAvatar))
  (UserInterface|Viewport|AddtoViewport _output_get 2)
  (Input|DisableInput (Game|GetPlayerCharacter 0) (Game|GetPlayerController 0)))

(event Collision|EventActorEndOverlap
  (params (OtherActor :type Actor%20Object%20Reference))
  ;[1 1 1] Pop up the dialog when player collide with the collider
  (Utilities|Casting|CastToCharacter OtherActor)
  (Widget|RemovefromParent (Variables|Default|GetDialogueBox)))

(fn ConstructionScript)