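; Door Blueprint tied to an NPC that swings open when that NPC is destroyed.
; The NPC's OnDestroyed event plays a timeline that drives the yaw of the Anchor component's relative rotation.
; Tick also compares the NPC's Response to ResponseToCheck, but the match only reaches a DoOnce with nothing wired after it.
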(event OnDestroyed(NPC)
  (params (DestroyedActor :type Actor%20Object%20Reference))
  (bind _rotation (Timeline|Timeline_0 Play)
    (:Update
      (Transformation|SetRelativeRotation (Variables|Default|GetAnchor) (Math|Rotator|MakeRotator 0.0 0.0 _rotation) false false))))

(event EventBeginPlay
  (|CallParentFunction))

(event Collision|EventActorBeginOverlap
  (params (OtherActor :type Actor%20Object%20Reference)))

(event EventTick
  (params (DeltaSeconds :type Float%20%28single-precision%29))
  (|CallParentFunction DeltaSeconds)
  (if (Utilities|Name|Equal(Name) (Variables|Default|GetResponse%20to%20Check) (Variables|/Game/Blueprints/NPC/NPC_Base.NPC_Base_C|GetResponse (Variables|Default|GetNPC)))
    (Utilities|FlowControl|DoOnce false)))

(fn ConstructionScript
  (|CallParentFunction))