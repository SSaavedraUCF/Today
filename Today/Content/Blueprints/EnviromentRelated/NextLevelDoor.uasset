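; NextLevelDoor is a lockable door that sends Player_Eve to the level named in LevelToChangeTo on overlap.
; While unlocked, the overlap adds a loading screen widget, waits briefly, then opens the level.
; A separate open event plays the OPENSESAME timeline, whose every update triggers the door sound, sets the Anchor's yaw from the curve and clears Locked.
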(event Custom|Spooky%20Open%20OOoooooOOOOoo
  (bind _door_open_rotation (Timeline|OPEN%20SESAME Play)
    (:Update
      (Audio|PlaySound2D "/Game/Sound/SFX/Door_Noises/door_close2.door_close2" 1.0 1.0 0.0 0 0)
      (Transformation|SetRelativeRotation (Variables|Default|GetAnchor) (Math|Rotator|MakeRotator 0.0 0.0 _door_open_rotation) false false)
      (Variables|Default|SetLocked? false))))

(event EventBeginPlay)

(event Collision|EventActorBeginOverlap
  (params (OtherActor :type Actor%20Object%20Reference))
  (if (not (Variables|Default|GetLocked?))
    (Utilities|Casting|CastToPlayer_Eve OtherActor)
    (bind _returnvalue (UserInterface|CreateWidget "/Game/Blueprints/LoadingScreen/W_LoadingScreen.W_LoadingScreen_C"))
    (UserInterface|Viewport|AddtoViewport _returnvalue 0)
    (Utilities|FlowControl|Delay 2.0)
    (Game|OpenLevel(byName) (Variables|Default|GetLevel%20to%20Change%20to))))

(event EventTick
  (params (DeltaSeconds :type Float%20%28single-precision%29)))

(fn ConstructionScript)