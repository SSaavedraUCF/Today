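; Clean_Counter is a cleanable counter prop that the player wipes with an Item_Towel.
; Towel overlap with its box sets Interactable and, until cleaned, shows a "Click to Clean!" Interact_Flower widget, removed when the towel leaves.
; The CleanedCounter event swaps the mesh material, marks the counter cleaned, removes the prompt and clears Interactable.
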(event OnComponentBeginOverlap(Box)
  (params (OverlappedComponent :type Primitive%20Component%20Object%20Reference) (OtherActor :type Actor%20Object%20Reference) (OtherComp :type Primitive%20Component%20Object%20Reference) (OtherBodyIndex :type Integer) (bFromSweep :type Boolean) (SweepResult :type Hit%20Result%20Structure%20%28by%20ref%29))
  ;[1 1 1] Sets Interactable/Brings up Text
  (Utilities|Casting|CastToItem_Towel OtherActor)
  (Variables|Default|SetInteractable true)
  (if (not (Variables|Default|GetCleanedCounter))
    (Variables|Default|GetCleaning%20Text
      (:then)
      (:else
        (bind _returnvalue (UserInterface|CreateWidget "/Game/Blueprints/Inventory/Widgets/Interact_Flower.Interact_Flower_C" 0 "Click to Clean!"))
        (bind _output_get (Variables|Default|SetCleaning%20Text _returnvalue))
        (UserInterface|Viewport|AddtoViewport _output_get 0)))))

(event OnComponentEndOverlap(Box)
  (params (OverlappedComponent :type Primitive%20Component%20Object%20Reference) (OtherActor :type Actor%20Object%20Reference) (OtherComp :type Primitive%20Component%20Object%20Reference) (OtherBodyIndex :type Integer))
  ;[1 1 1] Text is Gone
  (Utilities|Casting|CastToItem_Towel OtherActor)
  (bind _cleaning_text (Variables|Default|GetCleaning%20Text)
    (:then
      (Widget|RemovefromParent _cleaning_text)
      (Variables|Default|SetCleaning%20Text 0))
    (:else)))

(event Custom|Cleaned%20Counter
  ;[1 1 1] Changes Texture
  (Rendering|Material|SetMaterial (Variables|Default|GetStatic%20Mesh) 0 "/Game/Art/Geometry/Materials/Environment/Regular_Materials/Mat_Prop_Mirror1.Mat_Prop_Mirror1")
  (Variables|Default|SetCleanedCounter true)
  (Widget|RemovefromParent (Variables|Default|GetCleaning%20Text))
  (Variables|Default|SetCleaning%20Text 0)
  (Variables|Default|SetInteractable false))

(fn ConstructionScript)