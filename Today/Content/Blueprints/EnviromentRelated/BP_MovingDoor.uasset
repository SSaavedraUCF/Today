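; BP_MovingDoor is a door actor whose DoorClose event puts a warning sticky note on it and arms further note triggers.
; The event spawns Item_StickyNote_warning at a mesh socket, fills its text from door variables, attaches it and sets HasPictureFrame.
; It then enables collision on every TriggerBox_SpawnNote tagged "house".
; The door animation is still a PrintString placeholder.
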(event Custom|Door%20Close
  ;[1 1 1] Spawns, Sets Variables
  (bind _returnvalue (Game|SpawnActorfromClass "/Game/Blueprints/Inventory/Items/Day4/Item_StickyNote_warning.Item_StickyNote_warning_C" (Math|Transform|MakeTransform (Transformation|GetSocketLocation (Variables|Debug|GetStaticMeshComponent) "Sticky Note") (Transformation|GetActorRotation)) "Undefined" 0 "*Task Text 
*Goes 
*Here" "Full note, 
 
Text 
Goes 
Here 
 
 
XOXO, 
Seb" 0))
  (bind _output_get (Variables|Default|SetSticky%20Note _returnvalue))
  (Variables|/Game/Blueprints/Inventory/Items/Day4/Item_StickyNote_warning.Item_StickyNote_warning_C|SetFull%20Note%20Text _output_get (Variables|Default|GetText%20Variable))
  (Variables|/Game/Blueprints/Inventory/Items/Day4/Item_StickyNote_warning.Item_StickyNote_warning_C|SetTask%20Text _output_get (Variables|Default|GetTask%20Text))
  (Transformation|AttachComponentToComponent _output_get (Variables|Debug|GetStaticMeshComponent) "Sticky Note" "SnapToTarget" "SnapToTarget" "KeepRelative" true) ; Makes sure it stays attached TO the door
  (Development|PrintString "attach animation") ; replace with animation
  (Variables|Default|Sethas%20picture%20frame? true)
  ;[1 1 1] active triggerbox to spawn stickynote warnings
  (bind _outactors (Actor|GetAllActorsOfClasswithTag "/Game/Levels/Maps/TriggerBox_SpawnNote.TriggerBox_SpawnNote_C" "house"))
  (bind _array_element (Utilities|Array|ForEachLoopwithBreak _outactors)
    (:LoopBody
      (Collision|SetActorEnableCollision _array_element true))))

(event EventBeginPlay)

(event Collision|EventActorBeginOverlap
  (params (OtherActor :type Actor%20Object%20Reference)))

(event EventTick
  (params (DeltaSeconds :type Float%20%28single-precision%29)))

(fn ConstructionScript)