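; BP_Door is a swinging door that can start locked and is unlocked when Player_Eve carries Item_MomKey into its KeyBox.
; Unlocking shows a HUD notification, destroys "Unlock"-tagged descriptive objects, and swaps collision from KeyBox to Box inside that loop.
; Box overlap shows a use prompt and sets Interactable, both cleared on end overlap.
; The Opening event plays or reverses a timeline rotating Anchor's yaw, based on Interactable and Opened.
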(event OnComponentBeginOverlap(Box)
  (params (OverlappedComponent :type Primitive%20Component%20Object%20Reference) (OtherActor :type Actor%20Object%20Reference) (OtherComp :type Primitive%20Component%20Object%20Reference) (OtherBodyIndex :type Integer) (bFromSweep :type Boolean) (SweepResult :type Hit%20Result%20Structure%20%28by%20ref%29))
  (if (not (Variables|Default|GetLocked?))
    (Utilities|Casting|CastToPlayer_Eve OtherActor)
    (Variables|Default|SetInteractable? true)
    (bind _returnvalue (UserInterface|CreateWidget "/Game/Blueprints/Inventory/Widgets/Interact_Text.Interact_Text_C" 0 "Left-Click to Use Door")) ; Change Key
    (bind _output_get (Variables|Default|SetInteract%20Text _returnvalue))
    (UserInterface|Viewport|AddtoViewport _output_get 0)))

(event OnComponentBeginOverlap(KeyBox)
  (params (OverlappedComponent :type Primitive%20Component%20Object%20Reference) (OtherActor :type Actor%20Object%20Reference) (OtherComp :type Primitive%20Component%20Object%20Reference) (OtherBodyIndex :type Integer) (bFromSweep :type Boolean) (SweepResult :type Hit%20Result%20Structure%20%28by%20ref%29))
  (bind _asplayer_eve (Utilities|Casting|CastToPlayer_Eve OtherActor))
  (bind _isininventory (Default|InventoryQuery (Variables|/Game/PlayerBP/Blueprints/Player_Eve.Player_Eve_C|GetAC_Inventory _asplayer_eve) "/Game/Blueprints/Inventory/Items/Item_MomKey.Item_MomKey_C" 1))
  (if _isininventory
    (bind _asmy_player_controller (Utilities|Casting|CastToMyPlayerController (Game|GetPlayerController 0)))
    (bind _returnvalue (UserInterface|CreateWidget "/Game/Blueprints/Inventory/Widgets/W_Inventory_Notification.W_Inventory_Notification_C" 0 "Door has been unlocked"))
    (Class|VerticalBox|AddChildtoVerticalBox (Variables|/Game/W_Notif_List.W_Notif_List_C|GetNotifVerticalBox (Variables|/Game/Blueprints/Inventory/InventoryUI/UI_HUD.UI_HUD_C|GetW_Notif_List (Variables|/Game/Blueprints/Inventory/MyPlayerController.MyPlayerController_C|GetHUD%20Widget _asmy_player_controller))) _returnvalue)
    (Variables|Default|SetLocked? false)
    (bind _outactors (Actor|GetAllActorsOfClasswithTag "/Game/Blueprints/Dialogue/BP_DescriptiveObject.BP_DescriptiveObject_C" "Unlock"))
    (for _array_element _outactors
      (Actor|DestroyActor _array_element)
      (Collision|SetCollisionEnabled (Variables|Default|GetKey%20Box) "NoCollision")
      (Collision|SetCollisionEnabled (Variables|Default|GetBox) "QueryOnly"))))

(event EventBeginPlay
  (bind _key_box (Variables|Default|GetKey%20Box))
  (bind _box (Variables|Default|GetBox))
  (if (Variables|Default|GetLocked?)
    (Collision|SetCollisionEnabled _key_box "QueryOnly")
    (Collision|SetCollisionEnabled _box "NoCollision")
    (else
      (Collision|SetCollisionEnabled _key_box "NoCollision")
      (Collision|SetCollisionEnabled _box "QueryOnly"))))

(event EventTick
  (params (DeltaSeconds :type Float%20%28single-precision%29)))

(event EventOpening
  (params (Actor :type Actor%20Object%20Reference))
  (if (not (Variables|Default|GetLocked?))
    (if (Math|Boolean|NANDBoolean (Variables|Default|GetInteractable?) (Variables|Default|GetOpened?))
      (Variables|Default|SetOpened? true)
      (bind _rotation (Timeline|Open%20TL Play)
        (:Update
          (Transformation|SetRelativeRotation (Variables|Default|GetAnchor) (Math|Rotator|MakeRotator 0.0 0.0 _rotation) false false)))
      (else
        (Variables|Default|SetOpened? false)
        (Timeline|Open%20TL Reverse)))))

(event Collision|EventActorEndOverlap
  (params (OtherActor :type Actor%20Object%20Reference))
  (bind _interact_text (Variables|Default|GetInteract%20Text)
    (:then
      (Widget|RemovefromParent _interact_text)
      (Variables|Default|SetInteract%20Text 0)
      (Utilities|Casting|CastToPlayer_Eve OtherActor)
      (Variables|Default|SetInteractable? false))
    (:else)))

(fn ConstructionScript)