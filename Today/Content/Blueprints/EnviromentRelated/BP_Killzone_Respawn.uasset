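; BP_Killzone_Respawn is a kill zone actor that sends the player back to a respawn point.
; On BeginPlay it caches the world location and rotation of its SPAWNPOINT component.
; When a Player_Eve overlaps the actor, it teleports that player to the cached transform, with debug prints left in both events.
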(event EventBeginPlay
  (bind _spawn_point (Variables|Default|GetSPAWN%20POINT))
  (bind _output_get (Variables|Default|SetSpawn%20Zone (Transformation|GetWorldLocation _spawn_point)))
  (Variables|Default|SetFacing%20Point (Transformation|GetWorldRotation _spawn_point))
  (Development|PrintString (Utilities|String|ToString(Vector) _output_get)))

(event Collision|EventActorBeginOverlap
  (params (OtherActor :type Actor%20Object%20Reference))
  (Development|PrintString "Hello")
  (bind _asplayer_eve (Utilities|Casting|CastToPlayer_Eve OtherActor))
  (Transformation|Teleport _asplayer_eve (Variables|Default|GetSpawn%20Zone) (Variables|Default|GetFacing%20Point)))

(event EventTick
  (params (DeltaSeconds :type Float%20%28single-precision%29)))

(fn ConstructionScript)