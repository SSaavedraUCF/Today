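; BP_MomDoor is a level-exit door that requires Player_Eve to carry an Item_Sphere.
; Box overlap queries the inventory, shows a click-to-open prompt and sets IsInteractable; leaving removes the prompt but never clears the flag.
; Tick polls left mouse presses while the flag is set and opens the level named by the Destination enum.
; The LeftClick function is an empty, abandoned test with disconnected logic.
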(event OnComponentBeginOverlap(Box)
  (params (OverlappedComponent :type Primitive%20Component%20Object%20Reference) (OtherActor :type Actor%20Object%20Reference) (OtherComp :type Primitive%20Component%20Object%20Reference) (OtherBodyIndex :type Integer) (bFromSweep :type Boolean) (SweepResult :type Hit%20Result%20Structure%20%28by%20ref%29))
  ;[1 1 1] Happen when eve come close to the door
  ;;[1 1 1] Check if eve have the key
  (bind _asplayer_eve (Utilities|Casting|CastToPlayer_Eve OtherActor))
  (bind _isininventory (Default|InventoryQuery (Variables|/Game/PlayerBP/Blueprints/Player_Eve.Player_Eve_C|GetAC_Inventory _asplayer_eve) "/Game/Blueprints/Inventory/Items/Item_Sphere.Item_Sphere_C" 1))
  (if _isininventory
    ;;[1 1 1] Add interact text
    (bind _returnvalue (UserInterface|CreateWidget "/Game/Blueprints/Inventory/Widgets/Interact_Text.Interact_Text_C" 0 "Left Click to Open")) ; Left-Click?
    (bind _output_get (Variables|Default|SetInteract%20Text _returnvalue))
    (UserInterface|Viewport|AddtoViewport _output_get 0)
    (Variables|Default|SetIs%20Interactable? true)))

(event OnComponentEndOverlap(Box)
  (params (OverlappedComponent :type Primitive%20Component%20Object%20Reference) (OtherActor :type Actor%20Object%20Reference) (OtherComp :type Primitive%20Component%20Object%20Reference) (OtherBodyIndex :type Integer))
  ;[1 1 1] Happen when eve come close to the door
  ;;[1 1 1] Remove interact text when eve exit the collider
  (Utilities|Casting|CastToPlayer_Eve OtherActor)
  (Widget|RemovefromParent (Variables|Default|GetInteract%20Text))
  (Variables|Default|SetInteract%20Text 0))

(event EventBeginPlay)

(event EventTick
  (params (DeltaSeconds :type Float%20%28single-precision%29))
  ;[1 1 1] Teleport to next level (Dont put this on tick, seb fix this pls)
  (if (and (Variables|Default|GetIs%20Interactable?) (Game|Player|WasInputKeyJustPressed (Game|GetPlayerController 0) "LeftMouseButton"))
    (Development|PrintString "teleported to next lvl")
    (Game|OpenLevel(byName) (Utilities|String|StringToName (Utilities|String|EnumtoString (Variables|Default|GetDestination))))))

(event Input|MouseEvents|LeftMouseButton
  (params (Key :type Key%20Structure :default "None"))
  ;[1 1 1] Teleport to next level (Dont put this on tick, seb fix this pls)
)

(fn ConstructionScript)

(fn LeftClick)