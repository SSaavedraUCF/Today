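; BP_ClassroomDoor is a classroom door that swings open and closed on a timeline unless it is Locked.
; BeginPlay enables either KeyBox or Box query collision based on the lock state.
; When Player_Eve overlaps Box, it becomes Interactable and shows a left-click prompt, cleared on overlap end.
; The Opening event plays or reverses the Anchor's yaw timeline, based on a NAND of Interactable and Opened.
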(event OnComponentBeginOverlap(Box)
  (params (OverlappedComponent :type Primitive%20Component%20Object%20Reference) (OtherActor :type Actor%20Object%20Reference) (OtherComp :type Primitive%20Component%20Object%20Reference) (OtherBodyIndex :type Integer) (bFromSweep :type Boolean) (SweepResult :type Hit%20Result%20Structure%20%28by%20ref%29))
  (if (not (Variables|Default|GetLocked?))
    (Utilities|Casting|CastToPlayer_Eve OtherActor)
    (Variables|Default|SetInteractable? true)
    (bind _returnvalue (UserInterface|CreateWidget "/Game/Blueprints/Inventory/Widgets/Interact_Text.Interact_Text_C" 0 "Left-Click to Use Door")) ; Change Key
    (bind _output_get (Variables|Default|SetInteract%20Text _returnvalue))
    (UserInterface|Viewport|AddtoViewport _output_get 0)))

(event EventBeginPlay
  (bind _key_box (Variables|Default|GetKey%20Box))
  (bind _box (Variables|Default|GetBox))
  (if (Variables|Default|GetLocked?)
    (Collision|SetCollisionEnabled _key_box "QueryOnly")
    (Collision|SetCollisionEnabled _box "NoCollision")
    (else
      (Collision|SetCollisionEnabled _key_box "NoCollision")
      (Collision|SetCollisionEnabled _box "QueryOnly"))))

(event EventTick
  (params (DeltaSeconds :type Float%20%28single-precision%29)))

(event EventOpening
  (params (Actor :type Actor%20Object%20Reference))
  (if (not (Variables|Default|GetLocked?))
    (if (Math|Boolean|NANDBoolean (Variables|Default|GetInteractable?) (Variables|Default|GetOpened?))
      (Variables|Default|SetOpened? true)
      (bind _rotation (Timeline|Open%20TL Play)
        (:Update
          (Transformation|SetRelativeRotation (Variables|Default|GetAnchor) (Math|Rotator|MakeRotator 0.0 0.0 _rotation) false false)))
      (else
        (Variables|Default|SetOpened? false)
        (Timeline|Open%20TL Reverse)))))

(event Collision|EventActorEndOverlap
  (params (OtherActor :type Actor%20Object%20Reference))
  (bind _interact_text (Variables|Default|GetInteract%20Text)
    (:then
      (Widget|RemovefromParent _interact_text)
      (Variables|Default|SetInteract%20Text 0)
      (Utilities|Casting|CastToPlayer_Eve OtherActor)
      (Variables|Default|SetInteractable? false))
    (:else)))

(fn ConstructionScript)