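; BP_Door_day6_Whitney is a child door Blueprint that only opens or closes while AllowedToBeOpen is set.
; That flag gates both the parent's begin-overlap logic and the Opening event, which plays or reverses OpenTL to yaw Anchor, based on Interactable and Opened.
; End overlap removes InteractText and clears Interactable for Player_Eve, while BeginPlay is overridden empty, skipping the parent's.
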(event EventBeginPlay)

(event Collision|EventActorBeginOverlap
  (params (OtherActor :type Actor%20Object%20Reference))
  (if (Variables|Default|GetAllowed%20to%20be%20Open?)
    (|CallParentFunction OtherActor)))

(event EventTick
  (params (DeltaSeconds :type Float%20%28single-precision%29))
  (|CallParentFunction DeltaSeconds) ; This node is disabled and will not be called.\nDrag off pins to build functionality.
)

(event EventOpening
  (params (Actor :type Actor%20Object%20Reference))
  (if (Variables|Default|GetAllowed%20to%20be%20Open?)
    (if (Math|Boolean|NANDBoolean (Variables|Default|GetInteractable?) (Variables|Default|GetOpened?))
      (Variables|Default|SetOpened? true)
      (bind _rotation (Timeline|OpenTL Play)
        (:Update
          (Transformation|SetRelativeRotation (Variables|Default|GetAnchor) (Math|Rotator|MakeRotator 0.0 0.0 _rotation) false false)))
      (else
        (Variables|Default|SetOpened? false)
        (Timeline|OpenTL Reverse)))))

(event Collision|EventActorEndOverlap
  (params (OtherActor :type Actor%20Object%20Reference))
  (bind _interact_text (Variables|Default|GetInteract%20Text)
    (:then
      (Widget|RemovefromParent _interact_text)
      (Variables|Default|SetInteract%20Text 0)
      (Utilities|Casting|CastToPlayer_Eve OtherActor)
      (Variables|Default|SetInteractable? false))
    (:else)))

(fn ConstructionScript
  (|CallParentFunction))