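; BP_Door_Teleporter is a door actor that flags itself interactable for Player_Eve and relocates an actor when opened.
; Beginning an overlap with Player_Eve stores the player reference and sets Interactable, with no end-overlap reset in these graphs.
; The Opening event moves the actor passed to it to a hardcoded world origin, without sweep or teleport physics, and reads neither stored variable.
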(event EventBeginPlay
  (|CallParentFunction) ; This node is disabled and will not be called.\nDrag off pins to build functionality.
)

(event Collision|EventActorBeginOverlap
  (params (OtherActor :type Actor%20Object%20Reference))
  (bind _asplayer_eve (Utilities|Casting|CastToPlayer_Eve OtherActor))
  (Variables|Default|SetEve _asplayer_eve)
  (Variables|Default|SetInteractable? true))

(event EventTick
  (params (DeltaSeconds :type Float%20%28single-precision%29))
  (|CallParentFunction DeltaSeconds) ; This node is disabled and will not be called.\nDrag off pins to build functionality.
)

(event EventOpening
  (params (Actor :type Actor%20Object%20Reference))
  (Transformation|SetActorLocation Actor "0, 0, 0" false false))

(fn ConstructionScript
  (|CallParentFunction))