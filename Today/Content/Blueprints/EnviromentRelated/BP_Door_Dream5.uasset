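; Door Blueprint, apparently for the Dream5 level, that extends a parent interactable door with locking and a scripted spooky close.
; AllowedToBeOpen gates both the parent's overlap-begin logic and the Opening event, which plays or reverses a timeline rotating the Anchor's yaw.
; CloseDoorSpooky runs a separate closing timeline only when BathroomDoor is set, then plays a close sound.
; Tick also prints InteractText's display name every frame.
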(event Custom|Close%20Door%20Spooky
  (if (Variables|Default|GetBathroom%20Door?)
    (bind _close (Timeline|CloseTL Play)
      (:Update
        (Transformation|SetRelativeRotation (Variables|Default|GetAnchor) (Math|Rotator|MakeRotator 0.0 0.0 _close) false false))
      (:Finished
        (Audio|PlaySoundatLocation "/Game/Sound/SFX/door_close2-2.door_close2-2" (Transformation|GetActorLocation) "0, 0, 0" 1.0 1.0 0.0 0 0 0)))))

(event EventBeginPlay
  (|CallParentFunction))

(event Collision|EventActorBeginOverlap
  (params (OtherActor :type Actor%20Object%20Reference))
  (if (Variables|Default|GetAllowed%20to%20be%20Open?)
    (|CallParentFunction OtherActor)))

(event EventTick
  (params (DeltaSeconds :type Float%20%28single-precision%29))
  (|CallParentFunction DeltaSeconds)
  (Development|PrintString (Utilities|GetDisplayName (Variables|Default|GetInteract%20Text))))

(event EventOpening
  (params (Actor :type Actor%20Object%20Reference))
  (if (Variables|Default|GetAllowed%20to%20be%20Open?)
    (if (Math|Boolean|NANDBoolean (Variables|Default|GetInteractable?) (Variables|Default|GetOpened?))
      (Variables|Default|SetOpened? true)
      (bind _rotation (Timeline|OpenTL Play)
        (:Update
          (Transformation|SetRelativeRotation (Variables|Default|GetAnchor) (Math|Rotator|MakeRotator 0.0 0.0 _rotation) false false)))
      (else
        (Variables|Default|SetOpened? false)
        (Timeline|OpenTL Reverse)))))

(event Collision|EventActorEndOverlap
  (params (OtherActor :type Actor%20Object%20Reference))
  (|CallParentFunction OtherActor))

(fn ConstructionScript
  (|CallParentFunction))