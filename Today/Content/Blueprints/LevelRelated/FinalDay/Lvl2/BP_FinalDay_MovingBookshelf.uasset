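; BP_FinalDay_MovingBookshelf is an interactable bookshelf in Final Day level 2 that slides once it has enough books.
; Its collider enables input and shows an interact prompt while Player_Eve overlaps it.
; Each Interact release queries Eve's inventory for Book1 and increments the shelf count, without removing the item.
; Reaching the required count unlocks the shelf and plays a timeline that moves it; the per-count switch branches are empty.
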(event OnComponentBeginOverlap(Collider)
  (params (OverlappedComponent :type Primitive%20Component%20Object%20Reference) (OtherActor :type Actor%20Object%20Reference) (OtherComp :type Primitive%20Component%20Object%20Reference) (OtherBodyIndex :type Integer) (bFromSweep :type Boolean) (SweepResult :type Hit%20Result%20Structure%20%28by%20ref%29))
  (Utilities|Casting|CastToPlayer_Eve OtherActor)
  (Input|EnableInput (Game|GetPlayerController 0))
  (Variables|Default|SetInteractable? true)
  (bind _returnvalue (UserInterface|CreateWidget "/Game/Blueprints/Inventory/Widgets/Interact_Text.Interact_Text_C" 0 "Press E to Interact"))
  (bind _output_get (Variables|Default|SetInteract%20Text _returnvalue))
  (UserInterface|Viewport|AddtoViewport _output_get 0))

(event OnComponentEndOverlap(Collider)
  (params (OverlappedComponent :type Primitive%20Component%20Object%20Reference) (OtherActor :type Actor%20Object%20Reference) (OtherComp :type Primitive%20Component%20Object%20Reference) (OtherBodyIndex :type Integer))
  (Utilities|Casting|CastToPlayer_Eve OtherActor)
  (Variables|Default|SetInteractable? false)
  (bind _interact_text (Variables|Default|GetInteract%20Text)
    (:then
      (Widget|RemovefromParent _interact_text)
      (Variables|Default|SetInteract%20Text 0))
    (:else)))

(event Custom|Moving%20Bookshelf
  ;[1 1 1] Bookshelf moving
  (if (not (Variables|Default|GetLocked))
    (bind _move (Timeline|Moving%20TL Play)
      (:Update
        (Transformation|SetRelativeLocation (Variables|Default|GetBookshelf) _move false false)))))

(event EventBeginPlay
  (Variables|Default|SetBooksinShelf 0))

(event Collision|EventActorBeginOverlap
  (params (OtherActor :type Actor%20Object%20Reference)))

(event EventTick
  (params (DeltaSeconds :type Float%20%28single-precision%29)))

(event Input|ActionEvents|InputActionInteractButton
  (params (Key :type Key%20Structure :default "None"))
  (:Released
    (if (Variables|Default|GetInteractable?)
      (bind _returnvalue (Actor|GetActorOfClass "/Game/PlayerBP/Blueprints/Player_Eve.Player_Eve_C"))
      (bind _isininventory (Default|InventoryQuery (Variables|/Game/PlayerBP/Blueprints/Player_Eve.Player_Eve_C|GetAC_Inventory _returnvalue) "/Game/Blueprints/LevelRelated/FinalDay/Lvl2/Item_FinalDayLvl2_Book1.Item_FinalDayLvl2_Book1_C" 1)) ; Do we really need 3 types of Book BP's?
      (if _isininventory
        (switch int (Variables|Default|GetBooksinShelf)
          (:Default
            _)
          (:0
            _)
          (:1
            _)
          (:2
            _))
        (Math|Integer|IncrementInt (Variables|Default|GetBooksinShelf) ; Adds 1 to Book to Bookshelf
          (:%20%20
            (if (== (Variables|Default|GetBooksNeeded) (Variables|Default|GetBooksinShelf))
              (Variables|Default|SetLocked false)
              (CallFunction|MovingBookshelf))))))))

(fn ConstructionScript)