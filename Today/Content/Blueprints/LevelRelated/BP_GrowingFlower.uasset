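; BP_GrowingFlower is a flower actor the player waters with the Princess watering can to make it grow.
; Overlap between its collider and Item_WateringCan_Princess toggles an interactable flag and shows or removes a "Left Click to Water" prompt widget.
; Tick polls for a left click while interactable, then Grow plays a timeline that scales the actor, disables the watering collider and marks it grown.
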(event OnComponentBeginOverlap(Collider(WateringCan))
  (params (OverlappedComponent :type Primitive%20Component%20Object%20Reference) (OtherActor :type Actor%20Object%20Reference) (OtherComp :type Primitive%20Component%20Object%20Reference) (OtherBodyIndex :type Integer) (bFromSweep :type Boolean) (SweepResult :type Hit%20Result%20Structure%20%28by%20ref%29))
  (Utilities|Casting|CastToItem_WateringCan_Princess OtherActor)
  (Variables|Default|SetInteractable? true)
  (if (not (Variables|Default|GetGrown?))
    (bind _returnvalue (UserInterface|CreateWidget "/Game/Blueprints/Inventory/Widgets/Interact_Text.Interact_Text_C" 0 "Left Click to Water"))
    (bind _output_get (Variables|Default|SetInteract%20Text _returnvalue))
    (UserInterface|Viewport|AddtoViewport _output_get 0)))

(event OnComponentEndOverlap(Collider(WateringCan))
  (params (OverlappedComponent :type Primitive%20Component%20Object%20Reference) (OtherActor :type Actor%20Object%20Reference) (OtherComp :type Primitive%20Component%20Object%20Reference) (OtherBodyIndex :type Integer))
  (Utilities|Casting|CastToItem_WateringCan_Princess OtherActor)
  (Variables|Default|SetInteractable? false)
  (bind _interact_text (Variables|Default|GetInteract%20Text)
    (:then
      (Widget|RemovefromParent _interact_text)
      (Variables|Default|SetInteract%20Text 0))
    (:else)))

(event Custom|Grow
  (if (not (Variables|Default|GetGrown?))
    (bind _growing (Timeline|Growing Play)
      (:Update
        (Transformation|SetActorRelativeScale3D (Math|Vector|MakeVector _growing _growing _growing))
        (Collision|SetCollisionEnabled (Variables|Default|GetCollider%20%28Watering%20Can%29) "NoCollision")
        (Variables|Default|SetGrown? true)))))

(event EventBeginPlay)

(event Collision|EventActorBeginOverlap
  (params (OtherActor :type Actor%20Object%20Reference)))

(event EventTick
  (params (DeltaSeconds :type Float%20%28single-precision%29))
  (if (and (Variables|Default|GetInteractable?) (Game|Player|WasInputKeyJustPressed (Game|GetPlayerController 0) "LeftMouseButton"))
    (if (not (Variables|Default|GetGrown?))
      (CallFunction|Grow))))

(fn ConstructionScript)