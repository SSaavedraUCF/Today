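; Rotating cabinet actor for Dream 8 that also serves as a level exit.
; Its Rotate event plays a timeline that lerps the cabinet's relative rotation between start and end rotators.
; When Player_Eve overlaps the door collision while it is unlocked, it shows a loading screen widget and opens the configured level after a short delay.
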(event OnComponentBeginOverlap(DoorCollision)
  (params (OverlappedComponent :type Primitive%20Component%20Object%20Reference) (OtherActor :type Actor%20Object%20Reference) (OtherComp :type Primitive%20Component%20Object%20Reference) (OtherBodyIndex :type Integer) (bFromSweep :type Boolean) (SweepResult :type Hit%20Result%20Structure%20%28by%20ref%29))
  ;[1 1 1] Teleport to next lvl
  (if (not (Variables|Default|GetLocked?))
    (Utilities|Casting|CastToPlayer_Eve OtherActor)
    (bind _returnvalue (UserInterface|CreateWidget "/Game/Blueprints/LoadingScreen/W_LoadingScreen.W_LoadingScreen_C"))
    (UserInterface|Viewport|AddtoViewport _returnvalue 0)
    (Utilities|FlowControl|Delay 2.0)
    (Game|OpenLevel(byName) (Variables|Default|GetLevel%20to%20Change%20to))))

(event Custom|Rotate
  ;[1 1 1] Cabinet rotate
  (bind _cabinet (Timeline|CabinetRotating Play)
    (:Update
      (Transformation|SetRelativeRotation (Variables|Default|Getcabinet) (Math|Rotator|Lerp(Rotator) (Variables|Default|GetStartRotation) (Variables|Default|GetEndRotation) _cabinet) false false))))

(fn ConstructionScript)