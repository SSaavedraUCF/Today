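; Door trigger for the Whitney house on Day 6 that teleports Eve once her conversation with Whitney is done.
; On collider overlap it checks that NPC_Day6_WhitneyStart's response is "Interacted", then shows a "Left Click to Enter" widget.
; Teleport and door sound fire immediately on that overlap, as the left-click check is left unconnected.
; Leaving the collider removes the prompt and clears CanEnter.
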(event OnComponentBeginOverlap(Colliderbox)
  (params (OverlappedComponent :type Primitive%20Component%20Object%20Reference) (OtherActor :type Actor%20Object%20Reference) (OtherComp :type Primitive%20Component%20Object%20Reference) (OtherBodyIndex :type Integer) (bFromSweep :type Boolean) (SweepResult :type Hit%20Result%20Structure%20%28by%20ref%29))
  ;[1 1 1] Teleport text pop up / allow to teleport
  ;;[1 1 1] Checking if eve finished talking to withney
  (bind _returnvalue (Actor|GetActorOfClass "/Game/Blueprints/NPC/Day6/NPC_Day6_WhitneyStart.NPC_Day6_WhitneyStart_C"))
  (if (Utilities|Name|Equal(Name) (Variables|/Game/Blueprints/NPC/NPC_Base.NPC_Base_C|GetResponse _returnvalue) "Interacted")
    (Utilities|Casting|CastToPlayer_Eve OtherActor)
    (bind _returnvalue_2 (UserInterface|CreateWidget "/Game/Blueprints/Inventory/Widgets/Interact_Text.Interact_Text_C" 0 "Left Click to Enter"))
    (bind _output_get (Variables|Default|SetText%20Widget _returnvalue_2))
    (UserInterface|Viewport|AddtoViewport _output_get 0)
    (Variables|Default|SetCan%20Enter true)
    ;[1 1 1] Teleport Player on button press
    (Development|PrintString "Can enter")
    (if (Variables|Default|GetCan%20Enter)
      (Audio|PlaySound2D "/Game/Sound/SFX/door_close2.door_close2" 1.0 1.0 0.0 0 0)
      (Transformation|SetActorLocationAndRotation (Game|GetPlayerCharacter 0) (Variables|Default|GetTP%20Location) (Math|Conversions|RotationFromXVector (Variables|Default|GetTP%20Rotation))))))

(event OnComponentEndOverlap(Colliderbox)
  (params (OverlappedComponent :type Primitive%20Component%20Object%20Reference) (OtherActor :type Actor%20Object%20Reference) (OtherComp :type Primitive%20Component%20Object%20Reference) (OtherBodyIndex :type Integer))
  ;[1 1 1] Teleport text pop up / allow to teleport
  (Utilities|Casting|CastToPlayer_Eve OtherActor)
  (Widget|RemovefromParent (Variables|Default|GetText%20Widget))
  (Variables|Default|SetCan%20Enter false))

(event EventBeginPlay
  (bind _asplayer_eve (Utilities|Casting|CastToPlayer_Eve (Game|GetPlayerCharacter 0)))
  (Variables|Default|SetPlayer%20Ref _asplayer_eve))

(fn ConstructionScript)