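; Day 6 trigger that lets Eve put up the blanket fort once she holds the blanket and Whitney's dialogue response allows it.
; Collider overlap checks both conditions, then shows an E-key prompt and arms a flag; leaving removes the prompt.
; Tick polls for E, spawns Day6_PillowFort, disables the collider and destroys the counter stools.
; A leftover debug print notes that the fort's teleport destination needs changing.
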(event OnComponentBeginOverlap(Collider)
  (params (OverlappedComponent :type Primitive%20Component%20Object%20Reference) (OtherActor :type Actor%20Object%20Reference) (OtherComp :type Primitive%20Component%20Object%20Reference) (OtherBodyIndex :type Integer) (bFromSweep :type Boolean) (SweepResult :type Hit%20Result%20Structure%20%28by%20ref%29))
  ;[1 1 1] Checking to see if eve finished whitney dialogue tree and have the blanket
  (bind _asplayer_eve (Utilities|Casting|CastToPlayer_Eve OtherActor))
  (bind _isininventory (Default|InventoryQuery (Variables|/Game/PlayerBP/Blueprints/Player_Eve.Player_Eve_C|GetAC_Inventory _asplayer_eve) "/Game/Blueprints/Inventory/Items/Item_Day6_Blanket.Item_Day6_Blanket_C" 1))
  (bind _returnvalue (Actor|GetActorOfClass "/Game/Blueprints/NPC/Day6/NPC_Day6_Whitney_InRoom.NPC_Day6_Whitney_InRoom_C"))
  (if (and _isininventory (Utilities|Name|Equal(Name) (Variables|/Game/Blueprints/NPC/NPC_Base.NPC_Base_C|GetResponse _returnvalue) "Can spawn Blanket"))
    (bind _returnvalue_2 (UserInterface|CreateWidget "/Game/Blueprints/Inventory/Widgets/Interact_Text.Interact_Text_C" 0 "Press E to put up the Blanket Fort"))
    (bind _output_get (Variables|Default|SetText_Widget _returnvalue_2))
    (UserInterface|Viewport|AddtoViewport _output_get 0)
    (Variables|Default|SetAble%20To%20Spawn? true)))

(event OnComponentEndOverlap(Collider)
  (params (OverlappedComponent :type Primitive%20Component%20Object%20Reference) (OtherActor :type Actor%20Object%20Reference) (OtherComp :type Primitive%20Component%20Object%20Reference) (OtherBodyIndex :type Integer))
  ;[1 1 1] Checking to see if eve finished whitney dialogue tree and have the blanket
  (Utilities|Casting|CastToPlayer_Eve OtherActor)
  (Widget|RemovefromParent (Variables|Default|GetText_Widget))
  (Variables|Default|SetAble%20To%20Spawn? false))

(event EventTick
  (params (DeltaSeconds :type Float%20%28single-precision%29))
  ;[1 1 1] Spawn the blanket flort
  (if (and (Variables|Default|GetAble%20To%20Spawn?) (Game|Player|IsInputKeyDown (Game|GetPlayerController 0) "E"))
    (Game|SpawnActorfromClass "/Game/Blueprints/LevelRelated/Day6/Day6_PillowFort.Day6_PillowFort_C" (Variables|Default|GetSpawn%20Fort%20Location) "Undefined" 0 0)
    (Variables|Default|SetAble%20To%20Spawn? false)
    (Collision|SetCollisionEnabled (Variables|Default|GetCollider) "NoCollision")
    (Development|PrintString "SEB! u have to go into day6 pillow fort to change the teleport destination" true true "(R=0.084088,G=1.000000,B=0.000000,A=1.000000)" 5.0)
    (bind _returnvalue (Actor|GetActorOfClass "/Game/Blueprints/LevelRelated/Day6/Day6_CounterStools.Day6_CounterStools_C"))
    (Actor|DestroyActor _returnvalue)))

(fn ConstructionScript)