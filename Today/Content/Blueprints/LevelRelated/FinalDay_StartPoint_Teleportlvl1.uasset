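; Final-day start-point trigger actor that sends the player to another level after the talk with Andi in the neighborhood.
; A Box overlap looks up the Andi NPC and sets Interactable if its Response is "Finished Talking", without checking the overlapping actor or ever clearing the flag.
; Tick polls for a left mouse click while Interactable, then opens the level named by LevelName.
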(event OnComponentBeginOverlap(Box)
  (params (OverlappedComponent :type Primitive%20Component%20Object%20Reference) (OtherActor :type Actor%20Object%20Reference) (OtherComp :type Primitive%20Component%20Object%20Reference) (OtherBodyIndex :type Integer) (bFromSweep :type Boolean) (SweepResult :type Hit%20Result%20Structure%20%28by%20ref%29))
  ;[1 1 1] Allow to be teleport?
  (bind _returnvalue (Actor|GetActorOfClass "/Game/Blueprints/NPC/FinalDay/StartPoint/NPC_Andi_FinalDay_Neighborhood.NPC_Andi_FinalDay_Neighborhood_C"))
  (if (Utilities|Name|Equal(Name) (Variables|/Game/Blueprints/NPC/NPC_Base.NPC_Base_C|GetResponse _returnvalue) "Finished Talking")
    (bind _output_get (Variables|Default|SetInteractable? true))
    (Development|PrintString (Utilities|String|ToString(Boolean) _output_get))))

(event EventBeginPlay)

(event Collision|EventActorBeginOverlap
  (params (OtherActor :type Actor%20Object%20Reference)))

(event EventTick
  (params (DeltaSeconds :type Float%20%28single-precision%29))
  ;[1 1 1] Teleport to next lvl (still bad idea to put this on tick :( )
  (if (and (Variables|Default|GetInteractable?) (Game|Player|WasInputKeyJustPressed (Game|GetPlayerController 0) "LeftMouseButton"))
    (Development|PrintString "teleported to next lvl")
    (Game|OpenLevel(byName) (Variables|Default|GetLevel%20Name))))

(fn ConstructionScript)