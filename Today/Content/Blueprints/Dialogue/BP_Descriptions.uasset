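; Observable item Blueprint that shows Eve's description of an object in a dialogue widget.
; Player overlap with the Box shows an interact prompt unless a description box is already set.
; ObserveItem toggles the W_DialoguePH widget, filled with the name Eve, description text and reaction image.
; Tick removes the prompt while the box is valid; leaving the Box removes both widgets only if the description box is valid.
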(event OnComponentEndOverlap(Box)
  (params (OverlappedComponent :type Primitive%20Component%20Object%20Reference) (OtherActor :type Actor%20Object%20Reference) (OtherComp :type Primitive%20Component%20Object%20Reference) (OtherBodyIndex :type Integer))
  (Utilities|Casting|CastToPlayerBP OtherActor)
  (bind _description_box (Variables|Default|GetDescription%20Box)
    (:then
      (Widget|RemovefromParent _description_box)
      (Variables|Default|SetInteract%20Text%20Widget 0))
    (:else)))

(event OnComponentBeginOverlap(Box)
  (params (OverlappedComponent :type Primitive%20Component%20Object%20Reference) (OtherActor :type Actor%20Object%20Reference) (OtherComp :type Primitive%20Component%20Object%20Reference) (OtherBodyIndex :type Integer) (bFromSweep :type Boolean) (SweepResult :type Hit%20Result%20Structure%20%28by%20ref%29))
  (Utilities|Casting|CastToPlayerBP OtherActor)
  (Variables|Default|GetDescription%20Box
    (:then)
    (:else
      (bind _returnvalue (UserInterface|CreateWidget "/Game/Blueprints/Inventory/Interact_Text.Interact_Text_C" 0 (Variables|Default|GetInteract%20Text)))
      (bind _output_get (Variables|Default|SetInteract%20Text%20Widget _returnvalue))
      (UserInterface|Viewport|AddtoViewport _output_get 0))))

(event EventObserveItem
  (bind _description_box (Variables|Default|GetDescription%20Box)
    (:then
      (Widget|RemovefromParent _description_box)
      (Variables|Default|SetDescription%20Box 0))
    (:else
      (bind _returnvalue (UserInterface|CreateWidget "/Game/Blueprints/Dialogue/Widgets/W_DialoguePH.W_DialoguePH_C"))
      (bind _output_get (Variables|Default|SetDescription%20Box _returnvalue))
      (Utilities|FlowControl|Sequence
        (:then_0
          (Variables|/Game/Blueprints/Dialogue/Widgets/W_DialoguePH.W_DialoguePH_C|SetNameText _output_get "Eve"))
        (:then_1
          (Variables|/Game/Blueprints/Dialogue/Widgets/W_DialoguePH.W_DialoguePH_C|SetDialogueText _output_get (Variables|Default|GetDescription%20Text)))
        (:then_2
          (Variables|/Game/Blueprints/Dialogue/Widgets/W_DialoguePH.W_DialoguePH_C|SetAvatarImage _output_get (Variables|Default|GetEve%20Reaction))
          (UserInterface|Viewport|AddtoViewport _returnvalue 0))))))

(event EventTick
  (params (DeltaSeconds :type Float%20%28single-precision%29))
  (Variables|Default|GetDescription%20Box
    (:then
      (Widget|RemovefromParent (Variables|Default|GetInteract%20Text%20Widget)))
    (:else)))

(fn ConstructionScript)