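; Trigger actor that shows a single thought line from Eve in a dialogue widget when the player overlaps it.
; On overlap by Player_Eve it creates W_DialoguePH with her name, thought text and reaction avatar, then disables player character input.
; Tick polls the E key to close the widget, restore input and, if DisplayOnce is set, disable the trigger's collision.
; End overlap by any Character also removes the widget.
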(event EventTick
  (params (DeltaSeconds :type Float%20%28single-precision%29))
  ;[1 1 1] Disable Dialogue Widget and Disable Trigger Box Collision
  (bind _dialogue_widget (Variables|Default|GetDialogue%20Widget)
    (:then
      (if (Game|Player|WasInputKeyJustPressed (Game|GetPlayerController 0) "E")
        (Widget|RemovefromParent _dialogue_widget)
        (Variables|Default|SetDialogue%20Widget 0)
        (Input|EnableInput (Game|GetPlayerCharacter 0) (Game|GetPlayerController 0))
        (if (Variables|Default|GetDisplay%20Once)
          (Collision|SetActorEnableCollision false))))
    (:else)))

(event Collision|EventActorBeginOverlap
  (params (OtherActor :type Actor%20Object%20Reference))
  ;[1 1 1] Pop up the dialog when player collide with the collider
  (Utilities|Casting|CastToPlayer_Eve OtherActor)
  (bind _returnvalue (UserInterface|CreateWidget "/Game/Blueprints/Dialogue/Widgets/W_DialoguePH.W_DialoguePH_C"))
  (bind _output_get (Variables|Default|SetDialogue%20Widget _returnvalue))
  (Variables|/Game/Blueprints/Dialogue/Widgets/W_DialoguePH.W_DialoguePH_C|SetNameText _output_get "Eve")
  (Variables|/Game/Blueprints/Dialogue/Widgets/W_DialoguePH.W_DialoguePH_C|SetDialogueText _output_get (Variables|Default|GetThoughts%200))
  (Variables|/Game/Blueprints/Dialogue/Widgets/W_DialoguePH.W_DialoguePH_C|SetAvatarImage _output_get (Variables|Default|GetEve%20Reaction))
  (UserInterface|Viewport|AddtoViewport _returnvalue 2)
  (Input|DisableInput (Game|GetPlayerCharacter 0) (Game|GetPlayerController 0)))

(event Collision|EventActorEndOverlap
  (params (OtherActor :type Actor%20Object%20Reference))
  ;[1 1 1] Pop up the dialog when player collide with the collider
  (Utilities|Casting|CastToCharacter OtherActor)
  (bind _dialogue_widget (Variables|Default|GetDialogue%20Widget)
    (:then
      (Widget|RemovefromParent _dialogue_widget))
    (:else)))

(event EventBeginPlay)

(fn ConstructionScript)