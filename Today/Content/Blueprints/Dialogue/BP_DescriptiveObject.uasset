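; BP_DescriptiveObject is an examinable object that shows Eve's reaction portrait and description in a dialogue box.
; Its box overlap stores the Player_Eve reference and shows an interact prompt, and leaving removes both widgets.
; ObserveItem toggles the dialogue, swapping out the prompt and disabling character input on open, with no re-enable here.
; Items flagged significant also write their significance text into Eve's note.
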(event OnComponentEndOverlap(Box)
  (params (OverlappedComponent :type Primitive%20Component%20Object%20Reference) (OtherActor :type Actor%20Object%20Reference) (OtherComp :type Primitive%20Component%20Object%20Reference) (OtherBodyIndex :type Integer))
  (Utilities|Casting|CastToPlayer_Eve OtherActor)
  (Utilities|FlowControl|Sequence
    (:then_0
      (bind _interact_text (Variables|Default|GetInteract%20Text)
        (:then
          (Widget|RemovefromParent _interact_text))
        (:else)))
    (:then_1
      (bind _dialoguebox (Variables|Default|GetDialogueBox)
        (:then
          (Widget|RemovefromParent _dialoguebox))
        (:else)))))

(event OnComponentBeginOverlap(Box)
  (params (OverlappedComponent :type Primitive%20Component%20Object%20Reference) (OtherActor :type Actor%20Object%20Reference) (OtherComp :type Primitive%20Component%20Object%20Reference) (OtherBodyIndex :type Integer) (bFromSweep :type Boolean) (SweepResult :type Hit%20Result%20Structure%20%28by%20ref%29))
  (bind _asplayer_eve (Utilities|Casting|CastToPlayer_Eve OtherActor))
  (Variables|Default|SetEve _asplayer_eve)
  (bind _returnvalue (UserInterface|CreateWidget "/Game/Blueprints/Inventory/Widgets/Interact_Text.Interact_Text_C" 0 (Variables|Default|GetItemText)))
  (bind _output_get (Variables|Default|SetInteract%20Text _returnvalue))
  (UserInterface|Viewport|AddtoViewport _output_get 0))

(event EventObserveItem
  (bind _dialoguebox (Variables|Default|GetDialogueBox)
    (:then
      (Widget|RemovefromParent _dialoguebox)
      (Variables|Default|SetDialogueBox 0)
      (Variables|/Script/Engine.PlayerController|SetbShowMouseCursor (Game|GetPlayerController 0) false))
    (:else
      (bind _interact_text (Variables|Default|GetInteract%20Text)
        (:then
          (Widget|RemovefromParent _interact_text)
          (bind _returnvalue (UserInterface|CreateWidget "/Game/Blueprints/Dialogue/Widgets/W_DialoguePH.W_DialoguePH_C" (Game|GetPlayerController 0)))
          (bind _output_get (Variables|Default|SetDialogueBox _returnvalue))
          (Utilities|FlowControl|Sequence
            (:then_0
              (Variables|/Game/Blueprints/Dialogue/Widgets/W_DialoguePH.W_DialoguePH_C|SetAvatarImage _output_get (Variables|Default|GetEveReaction)))
            (:then_1
              (Variables|/Game/Blueprints/Dialogue/Widgets/W_DialoguePH.W_DialoguePH_C|SetNameText _output_get "Eve"))
            (:then_2
              (Variables|/Game/Blueprints/Dialogue/Widgets/W_DialoguePH.W_DialoguePH_C|SetDialogueText _output_get (Variables|Default|GetDescription))
              (UserInterface|Viewport|AddtoViewport _output_get 0)
              (Input|DisableInput (Game|GetPlayerCharacter 0) (Game|GetPlayerController 0))
              (if (Variables|Default|GetSignificant%20Item?)
                (Variables|/Game/PlayerBP/Blueprints/Player_Eve.Player_Eve_C|SetEve's%20Note (Variables|Default|GetEve) (Variables|Default|GetSignificance%20Text))))))
        (:else)))))

(fn ConstructionScript)