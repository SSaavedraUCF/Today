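; Inventory component that stores items in a fixed number of slots and toggles the inventory window for the Player_Eve pawn.
; On BeginPlay it sizes the slot array; adding puts non-stackable items in the first empty slot, while stackable items are not yet handled.
; Queries look for a single slot holding enough of an item class.
; Toggling adds or removes the HUD canvas widget, switching input mode, cursor and open flag.
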(event EventBeginPlay
  (CallFunction|PrepareInventory))

(event EventTick
  (params (DeltaSeconds :type Float%20%28single-precision%29)))

(fn ToggleInventory
  (bind _returnvalue (Game|Player|GetPlayerPawn 0))
  (bind _returnvalue_2 (Game|GetPlayerController 0))
  (bind _returnvalue_3 (Game|GetPlayerController 0))
  (Variables|Default|GetInventory%20Window
    (:then
      (bind _asplayer_eve (Utilities|Casting|CastToPlayer_Eve _returnvalue))
      (Variables|/Game/PlayerBP/Blueprints/Player_Eve.Player_Eve_C|SetInventoryOpen _asplayer_eve false)
      (Widget|RemovefromParent (Variables|Default|GetInventory%20Window))
      (Variables|Default|SetInventory%20Window 0)
      (Input|SetInputModeGameOnly _returnvalue_3)
      (Variables|/Script/Engine.PlayerController|SetbShowMouseCursor _returnvalue_3 false))
    (:else
      (bind _asplayer_eve_2 (Utilities|Casting|CastToPlayer_Eve _returnvalue))
      (Variables|/Game/PlayerBP/Blueprints/Player_Eve.Player_Eve_C|SetInventoryOpen _asplayer_eve_2 true)
      (bind _returnvalue_4 (UserInterface|CreateWidget "/Game/Blueprints/Inventory/InventoryUI/UI_Inventory_Window.UI_Inventory_Window_C" 0 self))
      (Variables|Default|SetInventory%20Window _returnvalue_4)
      (bind _asmy_player_controller (Utilities|Casting|CastToMyPlayerController (Game|GetPlayerController 0)))
      (bind _returnvalue_5 (Class|CanvasPanel|AddChildtoCanvas (Variables|/Game/Blueprints/Inventory/InventoryUI/UI_HUD.UI_HUD_C|GetHudCanvas (Variables|/Game/Blueprints/Inventory/MyPlayerController.MyPlayerController_C|GetHUD%20Widget _asmy_player_controller)) (Variables|Default|GetInventory%20Window)))
      (Class|CanvasPanelSlot|SetAutoSize _returnvalue_5 true)
      (Class|CanvasPanelSlot|SetAlignment _returnvalue_5 "(X=0.500000,Y=0.500000)")
      (Class|CanvasPanelSlot|SetAnchors _returnvalue_5 (Variables|Default|GetAnchors))
      (Input|SetInputModeGameandUI _returnvalue_2 (Variables|Default|GetInventory%20Window) "DoNotLock" false)
      (Variables|/Script/Engine.PlayerController|SetbShowMouseCursor _returnvalue_2 true))))

(fn AddtoInventory
  (params (ItemToAdd :type Slot%20Structure%20Structure))
  (if (not (.isstackable (.item ItemToAdd)))
    (CallFunction|CreateStack ItemToAdd)
    (return true)))

(fn PrepareInventory
  (Utilities|Array|Resize (Variables|Default|GetInventory) (Variables|Default|GetNumberOfSlots)))

(fn CreateStack
  (params (ItemToAdd :type Slot%20Structure%20Structure))
  (bind (_array_element _array_index) (Utilities|Array|ForEachLoopwithBreak (Variables|Default|GetInventory) :!label _label)
    (:LoopBody
      (if (<= (.quantity _array_element) 0)
        (LocalVariables|SetHasSpace true)
        (LocalVariables|SetIdentified%20Index _array_index)
        (goto _label Break)))
    (:Completed
      (if (LocalVariables|GetHasSpace)
        (Utilities|Array|SetArrayElem (Variables|Default|GetInventory) (LocalVariables|GetIdentified%20Index) ItemToAdd)
        (return true)
        (else
          (return false))))))

(fn InventoryQuery
  (params (Item%20Query :type Item%20Class%20Reference) (Query%20Amount :type Integer))
  (bind _array_element (Utilities|Array|ForEachLoopwithBreak (Variables|Default|GetInventory) :!label _label)
    (:LoopBody
      (bind _output_get (LocalVariables|SetSuccess (and (== (.Class (Utilities|Struct|BreakItem_Structure (.item _array_element))) Item%20Query) (>= (.quantity _array_element) Query%20Amount))))
      (if _output_get
        (goto _label Break)))
    (:Completed
      (return (LocalVariables|GetSuccess)))))