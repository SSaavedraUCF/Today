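; Player controller that owns the in-game HUD and updates its tool icon display.
; On BeginPlay it creates the UI_HUD widget and adds it to the viewport, skipping this when the current level is MainMenu_Final.
; The SetIcon event passes a new icon to the HUD's WTools sub-widget and plays that widget's animation.
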(event Custom|Set%20Icon
  (params (Tool%20Icon :type Texture%202D%20Object%20Reference))
  (bind _hud_widget (Variables|Default|GetHUD%20Widget))
  (bind _w_tools (Variables|/Game/Blueprints/Inventory/InventoryUI/UI_HUD.UI_HUD_C|GetW_Tools _hud_widget))
  (Variables|/Game/Blueprints/Inventory/Widgets/Tools/W_Tools.W_Tools_C|SetTool%20Icon _w_tools Tool%20Icon)
  (Default|PlayAnimation _w_tools))

(event EventBeginPlay
  (bind _returnvalue (Game|GetCurrentLevelName true))
  (if (not (Utilities|Enum|Equal(Enum) _returnvalue "MainMenu_Final"))
    (bind _returnvalue_2 (UserInterface|CreateWidget "/Game/Blueprints/Inventory/InventoryUI/UI_HUD.UI_HUD_C"))
    (bind _output_get (Variables|Default|SetHUD%20Widget _returnvalue_2))
    (UserInterface|Viewport|AddtoViewport _output_get 0)))

(fn ConstructionScript)