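; Actor component that holds a slot-based player inventory and toggles its window.
; On BeginPlay it sizes the slot array to NumberOfSlots; non-stackable items fill the first empty slot, with no full-inventory check.
; Stackable items are not yet handled.
; Toggling creates or removes the widget on the HUD canvas, switches input mode and sets InventoryOpen on the AdvancedDBP pawn.
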(event EventBeginPlay
  (CallFunction|PrepareInventory))

(event EventTick
  (params (DeltaSeconds :type Float%20%28single-precision%29)))

(fn ToggleInventory
  (bind _returnvalue (Game|Player|GetPlayerPawn 0))
  (Variables|Default|GetInventory%20Window
    (:then
      (bind _asadvanced_dbp (Utilities|Casting|CastToAdvancedDBP _returnvalue))
      (Variables|/Game/ThirdPersonBP/Blueprints/AdvancedDBP.AdvancedDBP_C|SetInventoryOpen _asadvanced_dbp false)
      (Widget|RemovefromParent (Variables|Default|GetInventory%20Window))
      (Variables|Default|SetInventory%20Window 0)
      (Input|SetInputModeGameOnly (Game|GetPlayerController 0)))
    (:else
      (bind _asadvanced_dbp_2 (Utilities|Casting|CastToAdvancedDBP _returnvalue))
      (Variables|/Game/ThirdPersonBP/Blueprints/AdvancedDBP.AdvancedDBP_C|SetInventoryOpen _asadvanced_dbp_2 true)
      (bind _returnvalue_2 (UserInterface|CreateWidget "/Game/Blueprints/Sebastian/Inventory/InventoryUI/UI_Inventory_Window.UI_Inventory_Window_C" 0 self))
      (Variables|Default|SetInventory%20Window _returnvalue_2)
      (bind _asmy_player_controller (Utilities|Casting|CastToMyPlayerController (Game|GetPlayerController 0)))
      (bind _returnvalue_3 (Class|CanvasPanel|AddChildtoCanvas (Variables|/Game/Blueprints/Sebastian/Inventory/InventoryUI/UI_HUD.UI_HUD_C|GetHudCanvas (Variables|/Game/Blueprints/Sebastian/Inventory/MyPlayerController.MyPlayerController_C|GetHUD%20Widget _asmy_player_controller)) (Variables|Default|GetInventory%20Window)))
      (Class|CanvasPanelSlot|SetAutoSize _returnvalue_3 true)
      (Class|CanvasPanelSlot|SetAlignment _returnvalue_3 "(X=0.500000,Y=0.500000)")
      (Class|CanvasPanelSlot|SetAnchors _returnvalue_3 (Variables|Default|GetAnchors))
      (Input|SetInputModeGameandUI (Game|GetPlayerController 0) (Variables|Default|GetInventory%20Window) "DoNotLock" true))))

(fn AddtoInventory
  (params (ItemToAdd :type Slot%20Structure%20Structure))
  (if (not (.isstackable (.item ItemToAdd)))
    (CallFunction|CreateStack ItemToAdd)
    (return true)))

(fn PrepareInventory
  (Utilities|Array|Resize (Variables|Default|GetInventory) (Variables|Default|GetNumberOfSlots)))

(fn CreateStack
  (params (ItemToAdd :type Slot%20Structure%20Structure))
  (bind _inventory (Variables|Default|GetInventory))
  (Utilities|Array|SetArrayElem _inventory (Utilities|Array|FindItem _inventory (Utilities|Struct|MakeSlot_Structure "(Name_2_C84C946E4FD33DE5DCBD778874CA1B4F=NSLOCTEXT(\"[FB5881384D62D4ECAE95B780D3EE917F]\", \"5923E8514508D02F9FB6FB80531CEBB8\", \"None\"),Description_20_5FE4B0FD41A7132C06947A8524D2C6F2=NSLOCTEXT(\"[FB5881384D62D4ECAE95B780D3EE917F]\", \"A7E1F40D410E46FBAADBF28947820727\", \"None\"),Thumbnail_8_644BF10048D7D9D5EAC5DFA138C2D3E3=None,IsStackable_5_6F9ED94D4594E5791239F38E8140896D=False,MaxStackSize_13_85F37A8C407A5D5C9A6BE9AF329A1173=3,IsConsumable_17_9F612BC44DA870790BEC68BC17FB3D35=False,Class_23_381419544973D475AAF72BA36D07ADC6=None)")) ItemToAdd))