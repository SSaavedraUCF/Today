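; Day 5 radio actor that lets Player_Eve briefly silence its background music.
; Its Box overlap enables input and shows an interact prompt for Eve, though input is enabled before the cast check; leaving reverses this.
; Pressing E in range mutes BGMusic, then restores it after a short delay.
; IsOn is never set false, so the turn-on branch goes unused and the radio cannot stay off.
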(event OnComponentBeginOverlap(Box)
  (params (OverlappedComponent :type Primitive%20Component%20Object%20Reference) (OtherActor :type Actor%20Object%20Reference) (OtherComp :type Primitive%20Component%20Object%20Reference) (OtherBodyIndex :type Integer) (bFromSweep :type Boolean) (SweepResult :type Hit%20Result%20Structure%20%28by%20ref%29))
  ;[1 1 1] Check if Eve can Interact/Bring Up Text
  (Input|EnableInput (Game|GetPlayerController 0))
  (Utilities|Casting|CastToPlayer_Eve OtherActor)
  (Variables|Default|SetInteractable? true)
  (bind _returnvalue (UserInterface|CreateWidget "/Game/Blueprints/Inventory/Widgets/Interact_Text.Interact_Text_C" 0 "Press E to Interact"))
  (bind _output_get (Variables|Default|SetInteract%20Text _returnvalue))
  (UserInterface|Viewport|AddtoViewport _output_get 0))

(event OnComponentEndOverlap(Box)
  (params (OverlappedComponent :type Primitive%20Component%20Object%20Reference) (OtherActor :type Actor%20Object%20Reference) (OtherComp :type Primitive%20Component%20Object%20Reference) (OtherBodyIndex :type Integer))
  ;[1 1 1] Check if Eve can Interact/Bring Up Text
  (Utilities|Casting|CastToPlayer_Eve OtherActor)
  (Variables|Default|SetInteractable? false)
  (bind _interact_text (Variables|Default|GetInteract%20Text)
    (:then
      (Widget|RemovefromParent _interact_text)
      (Variables|Default|SetInteract%20Text 0)
      (Input|DisableInput (Game|GetPlayerController 0)))
    (:else)))

(event EventBeginPlay
  (Variables|Default|SetIs%20On? true))

(event Input|KeyboardEvents|E
  (params (Key :type Key%20Structure))
  (:Pressed
    (if (Variables|Default|GetInteractable?)
      (if (Variables|Default|GetIs%20On?)
        (Audio|Components|Audio|SetVolumeMultiplier (Variables|Default|GetBG%20Music) 0.0 :!class /Script/Engine.AudioComponent) ; Turns Off
        (Utilities|FlowControl|Delay 5.0)
        (Audio|Components|Audio|SetVolumeMultiplier (Variables|Default|GetBG%20Music) 1.0 :!class /Script/Engine.AudioComponent)
        (Variables|Default|SetIs%20On? true)
        (else
          (Audio|Components|Audio|SetVolumeMultiplier (Variables|Default|GetBG%20Music) 1.0 :!class /Script/Engine.AudioComponent))))))

(fn ConstructionScript)