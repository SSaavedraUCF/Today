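; Prototype flower actor that the player can water with a watering can.
; When an Item_WateringCan overlaps its Box, it sets Interactable and, if not yet watered, shows an Interact_Flower click prompt, removed when the can leaves.
; The WateredFlower event only sets the Watered and Finished flags; the mesh material swap is left unconnected.
; Interactable is never cleared here.
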(event OnComponentBeginOverlap(Box)
  (params (OverlappedComponent :type Primitive%20Component%20Object%20Reference) (OtherActor :type Actor%20Object%20Reference) (OtherComp :type Primitive%20Component%20Object%20Reference) (OtherBodyIndex :type Integer) (bFromSweep :type Boolean) (SweepResult :type Hit%20Result%20Structure%20%28by%20ref%29))
  (Utilities|Casting|CastToItem_WateringCan OtherActor)
  (Variables|Default|SetInteractable true)
  (if (not (Variables|Default|GetWatered))
    (Variables|Default|GetWatering%20Text
      (:then)
      (:else
        (bind _returnvalue (UserInterface|CreateWidget "/Game/Blueprints/Inventory/Widgets/Interact_Flower.Interact_Flower_C" 0 "Click to Water!"))
        (bind _output_get (Variables|Default|SetWatering%20Text _returnvalue))
        (UserInterface|Viewport|AddtoViewport _output_get 0)))))

(event OnComponentEndOverlap(Box)
  (params (OverlappedComponent :type Primitive%20Component%20Object%20Reference) (OtherActor :type Actor%20Object%20Reference) (OtherComp :type Primitive%20Component%20Object%20Reference) (OtherBodyIndex :type Integer))
  (Utilities|Casting|CastToItem_WateringCan OtherActor)
  (bind _watering_text (Variables|Default|GetWatering%20Text)
    (:then
      (Widget|RemovefromParent _watering_text)
      (Variables|Default|SetWatering%20Text 0))
    (:else)))

(event Custom|WateredFlower
  (Variables|Default|SetWatered true)
  (Variables|Default|SetFinished true))

(event EventBeginPlay)

(event Collision|EventActorBeginOverlap
  (params (OtherActor :type Actor%20Object%20Reference)))

(event EventTick
  (params (DeltaSeconds :type Float%20%28single-precision%29)))

(fn ConstructionScript)