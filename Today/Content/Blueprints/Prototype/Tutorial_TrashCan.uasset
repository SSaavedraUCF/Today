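; Tutorial trash can prototype that reports to the NPC_Andi character when it is watered, judging by its WateredFlower event and response names.
; The event finds Andi by class and advances the Response value: "Watered" becomes "BothWatered", and any other value becomes "WaterGarbage".
; BeginPlay, overlap and Tick are disabled stubs, so all behavior depends on that event being called.
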(event EventBeginPlay
  (|CallParentFunction) ; This node is disabled and will not be called.\nDrag off pins to build functionality.
)

(event Collision|EventActorBeginOverlap
  (params (OtherActor :type Actor%20Object%20Reference))
  (|CallParentFunction OtherActor) ; This node is disabled and will not be called.\nDrag off pins to build functionality.
)

(event EventTick
  (params (DeltaSeconds :type Float%20%28single-precision%29))
  (|CallParentFunction DeltaSeconds) ; This node is disabled and will not be called.\nDrag off pins to build functionality.
)

(event EventWateredFlower
  (bind _returnvalue (Actor|GetActorOfClass "/Game/Blueprints/NPC/NPC_Andi.NPC_Andi_C"))
  (if (Utilities|Name|Equal(Name) (Variables|/Game/Blueprints/NPC/NPC_Base.NPC_Base_C|GetResponse _returnvalue) "Watered")
    (Variables|/Game/Blueprints/NPC/NPC_Base.NPC_Base_C|SetResponse _returnvalue "BothWatered")
    (else
      (Variables|/Game/Blueprints/NPC/NPC_Base.NPC_Base_C|SetResponse _returnvalue "WaterGarbage"))))

(fn ConstructionScript
  (|CallParentFunction))