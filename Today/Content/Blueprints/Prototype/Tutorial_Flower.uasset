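; Tutorial flower actor that the watering can item can water, advancing the tutorial NPC's response.
; Box overlap with the can sets Interactable and, if unwatered, shows a click-to-water widget, which is removed when the can leaves.
; The WateredFlower event, not called within this graph, swaps the mesh material, sets the watered flags and writes the new response directly onto NPC_Andi.
; Interactable is never cleared here.
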(event OnComponentBeginOverlap(Box)
  (params (OverlappedComponent :type Primitive%20Component%20Object%20Reference) (OtherActor :type Actor%20Object%20Reference) (OtherComp :type Primitive%20Component%20Object%20Reference) (OtherBodyIndex :type Integer) (bFromSweep :type Boolean) (SweepResult :type Hit%20Result%20Structure%20%28by%20ref%29))
  (Utilities|Casting|CastToItem_TutorialWateringCan OtherActor)
  (Variables|Default|SetInteractable true)
  (if (not (Variables|Default|GetWatered))
    (Variables|Default|GetWatering%20Text
      (:then)
      (:else
        (bind _returnvalue (UserInterface|CreateWidget "/Game/Blueprints/Inventory/Widgets/Interact_Flower.Interact_Flower_C" (Game|GetPlayerController 0) "Click to Water!"))
        (bind _output_get (Variables|Default|SetWatering%20Text _returnvalue))
        (UserInterface|Viewport|AddtoViewport _output_get 0)))))

(event OnComponentEndOverlap(Box)
  (params (OverlappedComponent :type Primitive%20Component%20Object%20Reference) (OtherActor :type Actor%20Object%20Reference) (OtherComp :type Primitive%20Component%20Object%20Reference) (OtherBodyIndex :type Integer))
  (Utilities|Casting|CastToItem_TutorialWateringCan OtherActor)
  (Variables|Default|GetWatering%20Text
    (:then
      (Widget|RemovefromParent (Variables|Default|GetWatering%20Text))
      (Variables|Default|SetWatering%20Text 0))
    (:else)))

(event Custom|WateredFlower
  (Rendering|Material|SetMaterial (Variables|Default|GetFlowerMesh) 0 (Variables|Default|GetMaterial))
  (Variables|Default|SetWatered true)
  (Variables|Default|SetFlower%201 true)
  (bind _returnvalue (Actor|GetActorOfClass "/Game/Blueprints/NPC/NPC_Andi.NPC_Andi_C"))
  (Variables|/Game/Blueprints/NPC/NPC_Base.NPC_Base_C|SetResponse _returnvalue "Watered"))

(event EventBeginPlay)

(event Collision|EventActorBeginOverlap
  (params (OtherActor :type Actor%20Object%20Reference)))

(event EventTick
  (params (DeltaSeconds :type Float%20%28single-precision%29)))

(fn ConstructionScript)