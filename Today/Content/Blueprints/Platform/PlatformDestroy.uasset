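; Crumbling platform that drops after Player_Eve overlaps it, then respawns.
; First contact plays a crumble sound, and after a delay the FALL timeline moves Platform's relative Z before the actor is hidden.
; After another delay, Respawn plays the Reset timeline, then repositions and unhides the platform and clears Touched.
; The shake timeline is never triggered, and the stored StartingPoint is not read.
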(event Custom|Respawn
  (bind _newtrack_0 (Timeline|Reset Play)
    (:Finished
      (Transformation|SetRelativeLocation (Variables|Default|GetPlatform) (Math|Vector|MakeVector 0.0 0.0 _newtrack_0) false false)
      (Rendering|SetActorHiddenInGame false)
      (Variables|Default|SetTouched false))))

(event EventBeginPlay
  (Variables|Default|SetStarting%20Point (Transformation|GetActorLocation)))

(event Collision|EventActorBeginOverlap
  (params (OtherActor :type Actor%20Object%20Reference))
  (Utilities|Casting|CastToPlayer_Eve OtherActor)
  (if (Variables|Default|GetTouched)
    _
    (else
      (Audio|PlaySound2D "/Game/Sound/SFX/crumble.crumble" 1.0 1.0 0.0 0 0)
      (Variables|Default|SetTouched true)))
  (Utilities|FlowControl|Delay 2.0)
  (bind _fall (Timeline|FALL PlayFromStart)
    (:Update
      (Transformation|SetRelativeLocation (Variables|Default|GetPlatform) (Math|Vector|MakeVector 0.0 0.0 _fall) false false))
    (:Finished
      (Rendering|SetActorHiddenInGame true)
      (Utilities|FlowControl|Delay 2.0)
      (CallFunction|Respawn))))

(event EventTick
  (params (DeltaSeconds :type Float%20%28single-precision%29)))

(fn ConstructionScript)