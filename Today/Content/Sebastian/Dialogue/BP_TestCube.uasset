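; BP_TestCube is a test interactable that toggles a dialogue box on screen.
; Its Interact event removes the stored DialogueWidget if valid, otherwise it creates a W_DialogueBox for player controller 0.
; After adding the new widget to the viewport, it copies its SetDialogueText and SetNameText variables into the widget's dialogue and name text.
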(event EventInteract
  (Utilities|IsValid (Variables|Default|GetDialogueWidget)
    (:Is%20Valid
      (Widget|RemovefromParent (Variables|Default|GetDialogueWidget))
      (Variables|Default|SetDialogueWidget 0))
    (:Is%20Not%20Valid
      (bind _returnvalue (UserInterface|CreateWidget "/Game/Sebastian/Dialogue/W_DialogueBox.W_DialogueBox_C" (Game|GetPlayerController 0)))
      (bind _output_get (Variables|Default|SetDialogueWidget _returnvalue))
      (UserInterface|Viewport|AddtoViewport _output_get 0)
      (Variables|/Game/Sebastian/Dialogue/W_DialogueBox.W_DialogueBox_C|SetDialogueText (Variables|Default|GetDialogueWidget) (Variables|Default|GetSetDialogueText))
      (Variables|/Game/Sebastian/Dialogue/W_DialogueBox.W_DialogueBox_C|SetNameText (Variables|Default|GetDialogueWidget) (Variables|Default|GetSetNameText)))))

(fn ConstructionScript)