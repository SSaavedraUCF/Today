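; Placeholder NPC Blueprint that hands its dialogue tree to its NPC_AI controller on BeginPlay and starts dialogue through that controller on Talk.
; An older data-table system remains: Dialogue_Create shows or updates a text widget using lines Dialogue_GetLine matches by conversation and line ID.
; This file never calls Dialogue_Create, and its row-gathering and "Press E" prompt logic are disconnected, though EndOverlap still removes the prompt.
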(event EventBeginPlay
  (bind _asnpc_ai (Utilities|Casting|CastToNPC_AI (AI|GetAIController self)))
  (Variables|/Game/Sebastian/Dialogue/NPC_AI.NPC_AI_C|SetDialogueTree _asnpc_ai (Variables|Default|GetDialogueTree)))

(event Collision|EventActorBeginOverlap
  (params (OtherActor :type Actor%20Object%20Reference)))

(event EventTalk
  (bind _asnpc_ai (Utilities|Casting|CastToNPC_AI (AI|GetAIController self)))
  (Default|StartDialogue _asnpc_ai))

(event Collision|EventActorEndOverlap
  (params (OtherActor :type Actor%20Object%20Reference))
  (Widget|RemovefromParent (Variables|Default|GetInteractText)))

(fn ConstructionScript)

(fn DialogueCreate
  ;[1 1 1] Checks to see if Widget is there
  (Utilities|IsValid (Variables|Default|GetDialogueBox)
    (:Is%20Valid
      ;[1 1 1] If widget is there, add text
      (bind _returnedline (CallFunction|DialogueGetLine))
      (if (not (Utilities|Text|TextIsEmpty _returnedline))
        (Variables|/Game/Sebastian/Dialogue/W_DialoguePH.W_DialoguePH_C|SetDialogueText (Variables|Default|GetDialogueBox) _returnedline)))
    (:Is%20Not%20Valid
      ;[1 1 1] Adds widget to the player's screen
      (bind _returnvalue (UserInterface|CreateWidget "/Game/Sebastian/Dialogue/W_DialoguePH.W_DialoguePH_C" (Game|GetPlayerController 0)))
      (bind _output_get (Variables|Default|SetDialogueBox _returnvalue))
      (UserInterface|Viewport|AddtoViewport _output_get 0)
      (bind _returnedline_2 (CallFunction|DialogueGetLine))
      (Variables|/Game/Sebastian/Dialogue/W_DialoguePH.W_DialoguePH_C|SetDialogueText (Variables|Default|GetDialogueBox) _returnedline_2)
      (Variables|/Game/Sebastian/Dialogue/W_DialoguePH.W_DialoguePH_C|SetNameText (Variables|Default|GetDialogueBox) (Variables|Default|GetsetNameText)))))

(fn DialogueGetLine
  (for _array_element (Variables|Default|GetMyDialogue)
    (bind _returnvalue (Utilities|GetDataTableRow "/Game/Sebastian/Dialogue/CSV_TestDialogue.CSV_TestDialogue" _array_element)
      (:then
        (if (and (== (.Conversation_ID (Utilities|Struct|BreakDialogueStructure _returnvalue)) (Variables|Default|GetConversation_ID)) (== (.Line_ID (Utilities|Struct|BreakDialogueStructure _returnvalue)) (Variables|Default|GetLineCurrent)))
          (Utilities|Array|Add (LocalVariables|GetReturnedLines) (.Dialogue (Utilities|Struct|BreakDialogueStructure _returnvalue)))))))
  (if (== (Utilities|Array|Length (LocalVariables|GetReturnedLines)) 1)
    (return (Utilities|Array|Get(acopy) (LocalVariables|GetReturnedLines)))
    (else
      (Widget|RemovefromParent (Variables|Default|GetDialogueBox))
      (Variables|Default|SetDialogueBox 0)
      (Variables|Default|SetLineCurrent 0))))